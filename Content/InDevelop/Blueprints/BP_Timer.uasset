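; BP_Timer is a timed random-event director that triggers blinks, camera shakes and a train event on the player.
; A looping one-second timer increments and prints a counter, and rising thresholds unlock random rolls, some behind delays.
; The rolls drive an eye blink through a timeline writing to the MPC_Blink parameter collection, a world camera shake at the player, or the character's TrainRandom playback.
; A blink also fires shortly after BeginPlay.
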(event Custom|IncreaseCounter
  ;[1 1 1] Counter and trigger event
  (Utilities|FlowControl|Sequence
    (:then_0
      (bind _output_get (Variables|Default|SetCounter (+ (Variables|Default|GetCounter) 1)))
      (Development|PrintString (Utilities|String|ToString(Integer) _output_get)))
    (:then_1
      (if (>= (Variables|Default|GetCounter) 30)
        (Utilities|FlowControl|Delay 6.0)
        (switch int (Math|Random|RandomIntegerinRange 0 4)
          (:0
            (CallFunction|CameraShake)))))
    (:then_2
      (if (>= (Variables|Default|GetCounter) 50)
        (switch int (Math|Random|RandomIntegerinRange 0 49)
          (:1
            (bind _asbp_fps_character_dev (Utilities|Casting|CastToBP_FPS_Character_Dev (Game|Player|GetPlayerPawn 0)))
            (Audio|Components|Audio|Play (Variables|/Game/InDevelop/Blueprints/BP_FPS_Character_Dev.BP_FPS_Character_Dev_C|GetTrainRandom _asbp_fps_character_dev) 0.0)))))
    (:then_3
      (if (>= (Variables|Default|GetCounter) 15)
        (Utilities|FlowControl|Delay 5.0)
        (switch int (Math|Random|RandomIntegerinRange 0 6)
          (:0
            (CallFunction|BlackEye)))))))

(event Custom|CameraShake
  ;[1 1 1] Events
  (Camera|PlayWorldCameraShake "/Game/InDevelop/Blueprints/BP_CameraShake.BP_CameraShake_C" (Transformation|GetActorLocation (Game|Player|GetPlayerPawn 0)) 1e+02 1e+03)
  (Development|PrintString "Shake"))

(event Custom|Black_Eye
  ;[1 1 1] Events
  (Development|PrintString "BlackEye")
  (bind _newtrack_0 (Timeline|Timeline PlayFromStart)
    (:Update
      (Rendering|Material|SetScalarParameterValue "/Game/InDevelop/Material/MPC_Blink.MPC_Blink" "EyeHardness" _newtrack_0 :!class /Script/Engine.KismetMaterialLibrary)
      (Rendering|Material|SetScalarParameterValue "/Game/InDevelop/Material/MPC_Blink.MPC_Blink" "AmountOpened" _newtrack_0 :!class /Script/Engine.KismetMaterialLibrary))))

(event EventBeginPlay
  ;[1 1 1] Counter and trigger event
  (Utilities|FlowControl|Sequence
    (:then_0
      (Utilities|FlowControl|Delay 2.0)
      (CallFunction|BlackEye))
    (:then_2
      (Utilities|Time|SetTimerbyEvent (delegate Custom|IncreaseCounter) 1.0 true))))

(fn ConstructionScript)