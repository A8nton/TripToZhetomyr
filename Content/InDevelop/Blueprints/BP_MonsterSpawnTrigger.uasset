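; Trigger actor that spawns monsters in train "Plackart" actors when the player overlaps it.
; On each player overlap, it loops over every actor tagged TrainPlackart and spawns a BP_Monster at that actor's MonsterPlackart-tagged component, with no one-shot guard.
; Four SetTransform helpers return transforms of the Note1 to Note4 components on the last iterated actor, but nothing in this Blueprint calls them.
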(event Collision|EventActorBeginOverlap
  (params (OtherActor :type Actor%20Object%20Reference))
  (bind _outactors (Actor|GetAllActorswithTag "TrainPlackart"))
  (bind _output_get (Variables|Default|SetArrayPlackart _outactors))
  (for _array_element _output_get
    (bind _output_get_2 (Variables|Default|SetArrayElmentPlackart _array_element))
    (if (== OtherActor (Game|GetPlayerCharacter 0))
      (Game|SpawnActorfromClass "/Game/InDevelop/Blueprints/BP_Monster.BP_Monster_C" (Math|Transform|MakeTransform (Transformation|GetWorldLocation (Utilities|Array|Get(acopy) (Actor|GetComponentsbyTag _output_get_2 "/Script/Engine.SceneComponent" "MonsterPlackart"))) (Transformation|GetWorldRotation (Utilities|Array|Get(acopy) (Actor|GetComponentsbyTag _output_get_2 "/Script/Engine.SceneComponent" "MonsterPlackart")))) "AlwaysSpawn" "MultiplyWithRoot" 0 0))))

(fn ConstructionScript)

(fn SetTransformOne
  (bind _arrayelmentplackart (Variables|Default|GetArrayElmentPlackart))
  (bind _returnvalue (Actor|GetComponentsbyTag _arrayelmentplackart "/Script/Engine.SceneComponent" "Note1"))
  (bind _output (Utilities|Array|Get(acopy) _returnvalue))
  (bind _returnvalue_2 (Transformation|GetWorldRotation _output))
  (bind _returnvalue_3 (Transformation|GetWorldLocation _output))
  (bind _returnvalue_4 (Math|Transform|MakeTransform _returnvalue_3 _returnvalue_2))
  (bind (_location _rotation _scale) (Math|Transform|BreakTransform _returnvalue_4))
  (return (Math|Transform|MakeTransform _location _rotation _scale)))

(fn SetTransformTwo
  (bind _arrayelmentplackart (Variables|Default|GetArrayElmentPlackart))
  (bind _returnvalue (Actor|GetComponentsbyTag _arrayelmentplackart "/Script/Engine.SceneComponent" "Note2"))
  (bind _output (Utilities|Array|Get(acopy) _returnvalue))
  (bind _returnvalue_2 (Transformation|GetWorldLocation _output))
  (bind _returnvalue_3 (Transformation|GetWorldRotation _output))
  (bind _returnvalue_4 (Math|Transform|MakeTransform _returnvalue_2 _returnvalue_3))
  (bind (_location _rotation _scale) (Math|Transform|BreakTransform _returnvalue_4))
  (return (Math|Transform|MakeTransform _location _rotation _scale)))

(fn SetTransformThree
  (bind _arrayelmentplackart (Variables|Default|GetArrayElmentPlackart))
  (bind _returnvalue (Actor|GetComponentsbyTag _arrayelmentplackart "/Script/Engine.SceneComponent" "Note3"))
  (bind _output (Utilities|Array|Get(acopy) _returnvalue))
  (bind _returnvalue_2 (Transformation|GetWorldRotation _output))
  (bind _returnvalue_3 (Transformation|GetWorldLocation _output))
  (bind _returnvalue_4 (Math|Transform|MakeTransform _returnvalue_3 _returnvalue_2))
  (bind (_location _rotation _scale) (Math|Transform|BreakTransform _returnvalue_4))
  (return (Math|Transform|MakeTransform _location _rotation _scale)))

(fn SetTransformFour
  (bind _arrayelmentplackart (Variables|Default|GetArrayElmentPlackart))
  (bind _returnvalue (Actor|GetComponentsbyTag _arrayelmentplackart "/Script/Engine.SceneComponent" "Note4"))
  (bind _output (Utilities|Array|Get(acopy) _returnvalue))
  (bind _returnvalue_2 (Transformation|GetWorldRotation _output))
  (bind _returnvalue_3 (Transformation|GetWorldLocation _output))
  (bind _returnvalue_4 (Math|Transform|MakeTransform _returnvalue_3 _returnvalue_2))
  (bind (_location _rotation _scale) (Math|Transform|BreakTransform _returnvalue_4))
  (return (Math|Transform|MakeTransform _location _rotation _scale)))