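; Chasing monster character that runs at the player and, on contact, triggers a death sequence ending in the main menu.
; Tick and pawn sensing drive AI MoveTo, with walk speed rising when the player is far away.
; BeginPlay attaches a NavMeshBoundsVolume to the monster and updates navigation, then destroys the monster after a short delay unless it has caught the player.
; Contact turns the player's view, disables input, then plays attack, scream and screen fade.
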(event OnSeePawn(PawnSensing)
  (params (Pawn :type Pawn%20Object%20Reference))
  (Variables|Default|SetIsSeing%20Player true)
  (CallFunction|FollowPlayer))

(event OnComponentBeginOverlap(Collision)
  (params (OverlappedComponent :type Primitive%20Component%20Object%20Reference) (OtherActor :type Actor%20Object%20Reference) (OtherComp :type Primitive%20Component%20Object%20Reference) (OtherBodyIndex :type Integer) (bFromSweep :type Boolean) (SweepResult :type Hit%20Result%20Structure%20%28by%20ref%29))
  (Variables|Default|SetIsTurning true)
  (Variables|Default|SetTargetRotation (Math|Rotator|FindLookatRotation (Transformation|GetActorLocation (Game|GetPlayerCharacter 0)) (Transformation|GetActorLocation)))
  (bind _asbp_fps_character_dev (Utilities|Casting|CastToBP_FPS_Character_Dev OtherActor))
  (if (Variables|Default|GetIsTurning)
    (CallFunction|TurningtoMonster)
    (Input|DisableInput _asbp_fps_character_dev 0)
    (Variables|Default|Setbtimetodestroy true)
    (Utilities|FlowControl|Delay 1.0)
    (if (not (Variables|Default|GetIsAttck))
      (Animation|PlayAnimMontage "/Game/InDevelop/Animations/AI/AttackMontage.AttackMontage" 1.0 "None")
      (Audio|PlaySound2D "/Game/InDevelop/Animations/AI/ArtemsAssets/ScreamBeforeDie.ScreamBeforeDie" 1.0 1.0 0.0 0 0)
      (Variables|Default|SetIsAttck true)
      (bind _returnvalue (UserInterface|CreateWidget "/Game/InDevelop/UI/ScreenFadeWidget.ScreenFadeWidget_C"))
      (bind _output_get (Variables|Default|SetFade%20Widget _returnvalue))
      (UserInterface|Viewport|AddtoViewport _output_get 0)
      (Default|PlayFAdeAnimation _output_get)
      (Utilities|FlowControl|Delay 2.8)
      (Variables|Default|SetIsAttck false)
      (Game|OpenLevel(byName) "main_menu_test"))))

(event Custom|Follow%20Player
  (if (Variables|Default|GetIsSeing%20Player)
    (AI|AIMoveTo self "0, 0, 0" (Game|GetPlayerCharacter 0) 7e+01 false)
    (else
      (Variables|Default|SetIsSeing%20Player false))))

(event Custom|Monster%20speed
  (bind _returnvalue (Transformation|GetActorLocation))
  (bind _returnvalue_2 (Game|GetPlayerCharacter 0))
  (bind _returnvalue_3 (Transformation|GetActorLocation _returnvalue_2))
  (bind _returnvalue_4 (Math|Vector|Distance(Vector) _returnvalue _returnvalue_3))
  (Variables|Default|SetDistance _returnvalue_4)
  (bind _output_get (Variables|Default|SetFarAway (> _returnvalue_4 1e+03)))
  (if _output_get
    (Variables|/Script/Engine.CharacterMovementComponent|SetMaxWalkSpeed (Variables|Character|GetCharacterMovement) 1e+03)
    (Variables|Default|SetFarAway true)
    (else
      (Variables|/Script/Engine.CharacterMovementComponent|SetMaxWalkSpeed (Variables|Character|GetCharacterMovement) 7e+02)
      (Variables|Default|SetFarAway false))))

(event Custom|MonsterStop
  (Components|Movement|StopMovementImmediately (Variables|Character|GetCharacterMovement)))

(event Custom|Monster%20scream
  (Utilities|FlowControl|Delay 8.0)
  (switch int (Math|Random|RandomIntegerinRange 0 2)
    (:0
      (Audio|PlaySound2D "/Game/InDevelop/Animations/AI/ArtemsAssets/MonsterScream1.MonsterScream1" 1.0 1.0 0.0 0 0))
    (:1
      (Audio|PlaySound2D "/Game/InDevelop/Animations/AI/ArtemsAssets/MonsterScream2.MonsterScream2" 1.0 1.0 0.0 0 0))
    (:2
      (Audio|PlaySound2D "/Game/InDevelop/Animations/AI/ArtemsAssets/MonsterScream3.MonsterScream3" 1.0 1.0 0.0 0 0)))
  (CallFunction|MonsterScream))

(event Custom|TurningToMonster
  (Pawn|SetControlRotation (Game|GetPlayerController 0) (Math|Interpolation|RInterpTo (Pawn|GetControlRotation :!class /Script/Engine.Pawn) (Variables|Default|GetTargetRotation) (Utilities|Time|GetWorldDeltaSeconds) 1e+02)))

(event EventTick
  (params (DeltaSeconds :type Float%20%28single-precision%29))
  (CallFunction|MonsterSpeed)
  (if (not (Variables|Default|GetIsSeing%20Player))
    (AI|AIMoveTo self "0, 0, 0" (Game|GetPlayerCharacter 0) 5.0 false)))

(event EventBeginPlay
  (Audio|PlaySound2D "/Game/InDevelop/Animations/AI/ArtemsAssets/MonsterScream1.MonsterScream1" 1.0 1.0 0.0 0 0)
  (bind _returnvalue (Actor|GetActorOfClass "/Script/NavigationSystem.NavMeshBoundsVolume"))
  (bind _output_get (Variables|Default|SetControlledNavMesh _returnvalue))
  (Transformation|AttachComponentToComponent _output_get (Variables|Default|GetNavMeshAttachmentPoint) "None" "KeepRelative" "KeepRelative" "KeepRelative" true)
  (Class|NavigationSystemV1|OnNavigationBoundsUpdated (Class|NavigationSystemV1|GetNavigationSystem))
  (Utilities|FlowControl|Delay 2.0)
  (if (not (Variables|Default|Getbtimetodestroy))
    (Actor|DestroyActor)))

(fn ConstructionScript)

(fn PlayFadeAnimation)