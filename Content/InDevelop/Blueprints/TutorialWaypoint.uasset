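; Tutorial waypoint actor that shows the player's distance to it on a StartWaypoint widget.
; Tick converts the pawn distance to whole meters and swaps the text to an LMB interact prompt within one meter.
; The actor destroys itself three seconds after something overlaps its Trigger, or immediately when an overlap ends.
; No interaction input is handled here.
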(event OnComponentBeginOverlap(Trigger)
  (params (OverlappedComponent :type Primitive%20Component%20Object%20Reference) (OtherActor :type Actor%20Object%20Reference) (OtherComp :type Primitive%20Component%20Object%20Reference) (OtherBodyIndex :type Integer) (bFromSweep :type Boolean) (SweepResult :type Hit%20Result%20Structure%20%28by%20ref%29))
  (Utilities|FlowControl|Delay 3.0)
  (Actor|DestroyActor))

(event OnComponentEndOverlap(Trigger)
  (params (OverlappedComponent :type Primitive%20Component%20Object%20Reference) (OtherActor :type Actor%20Object%20Reference) (OtherComp :type Primitive%20Component%20Object%20Reference) (OtherBodyIndex :type Integer))
  (Actor|DestroyActor))

(event EventBeginPlay
  (bind _asstart_waypoint (Utilities|Casting|CastToStartWaypoint (UserInterface|GetWidget (Variables|Default|GetWidget))))
  (Variables|Default|SetHow%20Long%20Text (Variables|/Game/InDevelop/UI/StartWaypoint.StartWaypoint_C|GetHowLongText _asstart_waypoint)))

(event EventTick
  (params (DeltaSeconds :type Float%20%28single-precision%29))
  (bind _returnvalue (Game|Player|GetPlayerPawn 0))
  (bind _returnvalue_2 (Transformation|GetActorLocation))
  (bind _how_long_text (Variables|Default|GetHow%20Long%20Text))
  (bind _returnvalue_3 (Transformation|GetActorLocation _returnvalue))
  (bind _returnvalue_4 (Math|Vector|Distance(Vector) _returnvalue_2 _returnvalue_3))
  (bind _returnvalue_5 (/ _returnvalue_4 1e+02))
  (Utilities|FlowControl|Sequence
    (:then_0
      (if (<= _returnvalue_5 1.0)
        (Rendering|Components|TextRender|SetText _how_long_text "Press LMB to Interact")
        (else
          (Rendering|Components|TextRender|SetText _how_long_text (Utilities|Text|ToText(String) (Utilities|String|Append (Utilities|String|ToString(Integer) (Math|Float|Truncate _returnvalue_5)) " m"))))))))

(fn ConstructionScript)