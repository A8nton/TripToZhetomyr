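; FinalWaypoint is a waypoint actor that shows the player's distance to it through a widget component.
; On BeginPlay it casts the widget to StartWaypoint and caches its HowLongText text block.
; Every Tick it converts the pawn distance to whole meters for display, switching to a "Press F to Interact" prompt at close range.
; It only displays the prompt and handles no input itself.
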(event EventBeginPlay
  (bind _asstart_waypoint (Utilities|Casting|CastToStartWaypoint (UserInterface|GetWidget (Variables|Default|GetWidget))))
  (Variables|Default|SetHow%20Long%20Text (Variables|/Game/InDevelop/UI/StartWaypoint.StartWaypoint_C|GetHowLongText _asstart_waypoint)))

(event EventTick
  (params (DeltaSeconds :type Float%20%28single-precision%29))
  (bind _returnvalue (Game|Player|GetPlayerPawn 0))
  (bind _returnvalue_2 (Transformation|GetActorLocation))
  (bind _how_long_text (Variables|Default|GetHow%20Long%20Text))
  (bind _returnvalue_3 (Transformation|GetActorLocation _returnvalue))
  (bind _returnvalue_4 (Math|Vector|Distance(Vector) _returnvalue_2 _returnvalue_3))
  (bind _returnvalue_5 (/ _returnvalue_4 1e+02))
  (if (<= _returnvalue_5 1.5)
    (Rendering|Components|TextRender|SetText _how_long_text "Press F to Interact")
    (else
      (Rendering|Components|TextRender|SetText _how_long_text (Utilities|Text|ToText(String) (Utilities|String|Append (Utilities|String|ToString(Integer) (Math|Float|Truncate _returnvalue_5)) " m"))))))

(fn ConstructionScript)