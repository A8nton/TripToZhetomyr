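; In-development first-person player character with stamina-based sprint, physics object handling, a three-slot food inventory and a dev menu.
; Camera traces highlight physics objects, feed a PhysicsHandle for holding and per-axis rotation, and store items as IDs read from actor tags.
; Eating the selected item, or pressing debug number keys, applies one timed speed or stamina effect at a time.
; The Main widget displays stamina, inventory, rotation axes and dev toggles.
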(event Custom|Food
  (params (FoodType :type Integer))
  ;[1 1 1] Food buffs
  (if (Variables|Food|GetisBuffActive)
    (Development|PrintString "Buff is now active")
    (else
      (Variables|Inventory|SetisInventoryAvailable true)
      (switch int FoodType
        (:1
          ;;[1 1 1] Beer Debuff - Decrease speed for 5 seconds
          (Development|PrintString "Beer debuff")
          (Variables|Food|SetisBuffActive true)
          (Variables|Moving|SetbaseSpeed 4e+02)
          (Variables|Moving|SetsprintSpeed 1e+03)
          (Utilities|FlowControl|Delay 5.0)
          (Development|PrintString "Beer debuff End")
          (Variables|Moving|SetbaseSpeed 6e+02)
          (Variables|Moving|SetsprintSpeed 1.5e+03)
          (Variables|Food|SetisBuffActive false))
        (:2
          ;;[1 1 1] Pizza buff - don't spend stamina for 5 seconds
          (Development|PrintString "Pizza buff")
          (Variables|Food|SetisBuffActive true)
          (Variables|Dev|Setdev_speed true)
          (Default|Num1 (Variables|UI|GetMain))
          (Utilities|FlowControl|Delay 5.0)
          (Development|PrintString "Pizza buff End")
          (Variables|Dev|Setdev_speed false)
          (Default|Num1 (Variables|UI|GetMain))
          (Variables|Food|SetisBuffActive false))
        (:3
          ;;[1 1 1] Burger buff - stamina regen 2x for 10 seconds
          (Development|PrintString "Burger buff")
          (Variables|Food|SetisBuffActive true)
          (Variables|Moving|SetstaminaRegen 2.0)
          (Utilities|FlowControl|Delay 1e+01)
          (Development|PrintString "Burger buff End")
          (Variables|Moving|SetstaminaRegen 1.0)
          (Variables|Food|SetisBuffActive false))
        (:4
          ;;[1 1 1] Cola buff - run faster for 5 seconds
          (Development|PrintString "Cola buff")
          (Variables|Food|SetisBuffActive true)
          (Variables|Moving|SetsprintSpeed 2e+03)
          (Utilities|FlowControl|Delay 5.0)
          (Development|PrintString "Cola buff End")
          (Variables|Moving|SetsprintSpeed 1.5e+03)
          (CallFunction|StopSprint)
          (Variables|Food|SetisBuffActive false))))))

(event EventTick
  (params (DeltaSeconds :type Float%20%28single-precision%29))
  (bind _pixelperfectcamera (Variables|Components|GetPixelPerfectCamera))
  (bind _holdingobjectrotation (Variables|Pickup|GetholdingObjectRotation))
  (bind _main (Variables|UI|GetMain))
  (bind _returnvalue (Transformation|GetWorldLocation _pixelperfectcamera))
  ;[1 1 1] Character
  ;;[1 1 1] Stamina Recharge
  (Utilities|FlowControl|Sequence
    (:then_0
      (Utilities|FlowControl|Delay 0.15)
      (if (Variables|Dev|Getdev_speed)
        (if (< (Variables|Moving|GetsprintStamina) 1e+02) :!label _label
          (bind _output_get (Variables|Moving|SetsprintStamina (+ (Variables|Moving|GetsprintStamina) (Variables|Moving|GetstaminaRegen))))
          (Default|UIUpdateStamina (Variables|UI|GetMain) _output_get 1e+02)
          ;;[1 1 1] Stamina Consumption
          (Widget|SetVisibility (Variables|/Game/InDevelop/UI/Main.Main_C|GetPROG_Stamina (Variables|UI|GetMain)) "Visible"))
        (elif (not (Variables|Moving|GetIsSprint))
          (goto _label))))
    (:then_1
      (if (< (Variables|Moving|GetsprintStamina) 1.0)
        (Variables|Moving|SetIsSprint false)
        (CallFunction|StopSprint)))
    (:then_2
      (if (== (Variables|Moving|GetsprintStamina) 1e+02)
        (Utilities|FlowControl|Delay 0.5)
        (Widget|SetVisibility (Variables|/Game/InDevelop/UI/Main.Main_C|GetPROG_Stamina (Variables|UI|GetMain)) "Hidden")))
    (:then_3
      (Utilities|FlowControl|Sequence
        (:then_0
          ;[1 1 1] Holding and rotating object
          (Utilities|FlowControl|Sequence
            (:then_0
              (if (Variables|Pickup|GetisHoldingSmth)
                (if (stale Input|MouseEvents|LeftMouseButton _returnvalue_2)
                  (Utilities|FlowControl|Sequence
                    (:then_0
                      (if (== _holdingobjectrotation 0)
                        (Transformation|SetRelativeRotation (stale Input|MouseEvents|LeftMouseButton _output_get) (Math|Rotator|MakeRotator (stale Input|MouseEvents|MouseWheelUp _output_get) 0.0 0.0) false false)
                        (Widget|SetVisibility (Variables|/Game/InDevelop/UI/Main.Main_C|GetAxisXBorder _main) "Visible")
                        (elif (== _holdingobjectrotation 1)
                          (Transformation|SetRelativeRotation (stale Input|MouseEvents|LeftMouseButton _output_get) (Math|Rotator|MakeRotator 0.0 (stale Input|MouseEvents|MouseWheelDown _output_get) 0.0) false false)
                          (Widget|SetVisibility (Variables|/Game/InDevelop/UI/Main.Main_C|GetAxisYBorder _main) "Visible")
                          (else
                            (Transformation|SetRelativeRotation (stale Input|MouseEvents|LeftMouseButton _output_get) (Math|Rotator|MakeRotator 0.0 0.0 (stale Input|MouseEvents|MouseWheelDown _output_get)) false false)
                            (Widget|SetVisibility (Variables|/Game/InDevelop/UI/Main.Main_C|GetAxisZBorder _main) "Visible")))))
                    (:then_1
                      (Class|PrimitiveComponent|SetPhysicsAngularVelocityinRadians (stale Input|MouseEvents|LeftMouseButton _output_get) "0, 0, 0" false "None"))
                    (:then_2
                      (if (> (Class|KismetMathLibrary|VectorDistanceSquared (Transformation|GetWorldLocation (Variables|Components|GetPixelPerfectCamera)) (Transformation|GetWorldLocation (.HitComponent (Collision|BreakHitResult (stale Input|MouseEvents|LeftMouseButton _outhit))))) 4.5e+04)
                        (Physics|Components|PhysicsHandle|ReleaseComponent (Variables|Default|GetPhysicsHandle))
                        (Utilities|FlowControl|Sequence
                          (:then_0
                            (Variables|Pickup|SetisHoldingSmth false)
                            (Variables|Pickup|SetheldObgectRotation 0.0)
                            (Widget|SetVisibility (Variables|/Game/InDevelop/UI/Main.Main_C|GetAxisXBorder (Variables|UI|GetMain)) "Hidden")))))))))
            (:then_1
              (if (stale _returnvalue_2)
                (Rendering|SetRenderCustomDepth (.HitComponent (Collision|BreakHitResult (stale _outhit))) false)))))
        (:then_1
          (bind (_outhit _returnvalue_2) (Collision|LineTraceByChannel _returnvalue (+ (* (Math|Vector|GetForwardVector _pixelperfectcamera) (Variables|Pickup|GetPickupDIstance)) _returnvalue) "TraceTypeQuery1" false 0 "None"))
          (if _returnvalue_2
            (if (Physics|IsSimulatingPhysics (Variables|/Script/Engine.Actor|GetRootComponent (.HitActor (Collision|BreakHitResult _outhit))) "None")
              (Rendering|SetRenderCustomDepth (.HitComponent (Collision|BreakHitResult _outhit)) true))))))))

(event EventBeginPlay
  ;[1 1 1] Widgets
  (Utilities|FlowControl|Sequence
    (:then_1
      (bind _returnvalue (UserInterface|CreateWidget "/Game/InDevelop/UI/Main.Main_C" (Game|GetPlayerController 0)))
      (bind _output_get (Variables|UI|SetMain _returnvalue))
      (UserInterface|Viewport|AddtoViewport _output_get 0)
      (Widget|SetVisibility (Variables|UI|GetMain) "Visible")
      (Utilities|FlowControl|Sequence
        (:then_0
          (Widget|SetVisibility (Variables|/Game/InDevelop/UI/Main.Main_C|GetDevMenu_Widget (Variables|UI|GetMain)) "Hidden"))
        (:then_1
          (Widget|SetVisibility (Variables|/Game/InDevelop/UI/Main.Main_C|GetInventoryOverlay (Variables|UI|GetMain)) "Hidden"))))))

(event Input|ActionEvents|InputActionSprint
  (params (Key :type Key%20Structure :default "None"))
  ;[1 1 1] Character
  ;;[1 1 1] Sprint
  (:Pressed
    (if (Variables|Moving|GetisMoving)
      (if (> (Variables|Moving|GetsprintStamina) 0.0)
        (CallFunction|StartSprint)
        (else
          (CallFunction|StopSprint :!label _label)))))
  (:Released
    (goto _label)))

(event Input|ActionEvents|InputActionSprint
  (params (Key :type Key%20Structure :default "None"))
  ;[1 1 1] DevThings
  ;;[1 1 1] Dev inf Sprint
  (:Pressed
    (switch Utilities|FlowControl|Switch|SwitchonECheckBoxState (Class|CheckBox|GetCheckedState (Variables|/Game/InDevelop/UI/Main.Main_C|Getwb_sprint (Variables|UI|GetMain))) :!label _label
      (:Unchecked
        (Variables|Dev|Setdev_speed false))
      (:Checked
        (Variables|Dev|Setdev_speed true))))
  (:Released
    (goto _label)))

(event Input|ActionEvents|InputActionIsMoving
  (params (Key :type Key%20Structure :default "None"))
  ;[1 1 1] Character
  ;;[1 1 1] Sprint
  (:Pressed
    (Variables|Moving|SetisMoving true))
  (:Released
    (Variables|Moving|SetisMoving false)))

(event Input|ActionEvents|InputActionJump
  (params (Key :type Key%20Structure :default "None"))
  ;[1 1 1] DevThings
  ;;[1 1 1] Dev Jump
  (:Pressed
    (if (Variables|Dev|Getwb_jump)
      (Character|Jump))))

(event Input|AxisEvents|InputAxisTurn
  (params (AxisValue :type Float%20%28single-precision%29))
  (bind _pixelperfectcamera (Variables|Components|GetPixelPerfectCamera))
  ;[1 1 1] Character
  ;;[1 1 1] Camera
  (Pawn|Input|AddControllerYawInput AxisValue)
  (Physics|Components|PhysicsHandle|SetTargetLocation (Variables|Default|GetPhysicsHandle) (+ (* (Math|Vector|GetForwardVector _pixelperfectcamera) (Variables|Pickup|GetHoldDistance)) (Transformation|GetWorldLocation _pixelperfectcamera))))

(event Input|AxisEvents|InputAxisLookUp
  (params (AxisValue :type Float%20%28single-precision%29))
  (bind _pixelperfectcamera (Variables|Components|GetPixelPerfectCamera))
  ;[1 1 1] Character
  ;;[1 1 1] Camera
  (Pawn|Input|AddControllerPitchInput AxisValue)
  (Physics|Components|PhysicsHandle|SetTargetLocation (Variables|Default|GetPhysicsHandle) (+ (* (Math|Vector|GetForwardVector _pixelperfectcamera) (Variables|Pickup|GetHoldDistance)) (Transformation|GetWorldLocation _pixelperfectcamera))))

(event Input|AxisEvents|InputAxisMoveForward
  (params (AxisValue :type Float%20%28single-precision%29))
  ;[1 1 1] Character
  ;;[1 1 1] Movement
  (Pawn|Input|AddMovementInput (Math|Vector|GetForwardVector (Variables|Collision|GetCapsuleComponent)) AxisValue false))

(event Input|AxisEvents|InputAxisMoveRight
  (params (AxisValue :type Float%20%28single-precision%29))
  ;[1 1 1] Character
  ;;[1 1 1] Movement
  (Pawn|Input|AddMovementInput (Math|Vector|GetRightVector (Variables|Collision|GetCapsuleComponent)) AxisValue false))

(event Input|AxisEvents|InputAxisMoveForward
  (params (AxisValue :type Float%20%28single-precision%29))
  ;[1 1 1] Character
  ;;[1 1 1] Stamina Consumption
  (if (not (Variables|Dev|Getdev_speed))
    (Utilities|FlowControl|Delay 0.02)
    (if (Variables|Moving|GetIsSprint)
      (bind _output_get (Variables|Moving|SetsprintStamina (- (Variables|Moving|GetsprintStamina) 1.0)))
      (Default|UIUpdateStamina (Variables|UI|GetMain) _output_get 1e+02)
      (Widget|SetVisibility (Variables|/Game/InDevelop/UI/Main.Main_C|GetPROG_Stamina (Variables|UI|GetMain)) "Visible"))))

(event Input|KeyboardEvents|Q
  (params (Key :type Key%20Structure :default "None"))
  ;[1 1 1] DevThings
  ;;[1 1 1] DevMenu
  (:Pressed
    (if (Variables|Dev|GetisInDev)
      (Variables|Dev|SetisInDev false)
      (CallFunction|DevMenuOff)
      (else
        (Variables|Dev|SetisInDev true)
        (CallFunction|DevMenuon)))))

(event Input|KeyboardEvents|NumPadOne
  (params (Key :type Key%20Structure :default "None"))
  ;[1 1 1] DevThings
  ;;[1 1 1] Dev inf Sprint
  (:Pressed
    (Default|Num1 (Variables|UI|GetMain))))

(event Input|MouseEvents|MouseWheelUp
  (params (Key :type Key%20Structure :default "None"))
  ;[1 1 1] Holding and rotating object
  (:Pressed
    (bind _output_get (Variables|Pickup|SetheldObgectRotation (+ (Variables|Pickup|GetheldObgectRotation) 2e+01)))))

(event Input|MouseEvents|MouseWheelDown
  (params (Key :type Key%20Structure :default "None"))
  ;[1 1 1] Holding and rotating object
  (:Pressed
    (bind _output_get (Variables|Pickup|SetheldObgectRotation (- (Variables|Pickup|GetheldObgectRotation) 2e+01)))))

(event Input|KeyboardEvents|1
  (params (Key :type Key%20Structure :default "None"))
  ;[1 1 1] DevThings
  ;;[1 1 1] Dev Foodbuffs initiation
  (:Pressed
    (bind _output_get (Variables|Food|SetFoodBuff 1))
    (CallFunction|Food _output_get)))

(event Input|KeyboardEvents|2
  (params (Key :type Key%20Structure :default "None"))
  ;[1 1 1] DevThings
  ;;[1 1 1] Dev Foodbuffs initiation
  (:Pressed
    (bind _output_get (Variables|Food|SetFoodBuff 2))
    (CallFunction|Food _output_get)))

(event Input|KeyboardEvents|3
  (params (Key :type Key%20Structure :default "None"))
  ;[1 1 1] DevThings
  ;;[1 1 1] Dev Foodbuffs initiation
  (:Pressed
    (bind _output_get (Variables|Food|SetFoodBuff 3))
    (CallFunction|Food _output_get)))

(event Input|KeyboardEvents|4
  (params (Key :type Key%20Structure :default "None"))
  ;[1 1 1] DevThings
  ;;[1 1 1] Dev Foodbuffs initiation
  (:Pressed
    (bind _output_get (Variables|Food|SetFoodBuff 4))
    (CallFunction|Food _output_get)))

(event Input|KeyboardEvents|W
  (params (Key :type Key%20Structure :default "None"))
  ;[1 1 1] Character
  ;;[1 1 1] Movement
  (:Released
    (CallFunction|StopSprint)))

(event Input|MouseEvents|RightMouseButton
  (params (Key :type Key%20Structure :default "None"))
  (bind _main (Variables|UI|GetMain))
  (bind _inventoryselect (Variables|Inventory|GetInventorySelect))
  (bind _inventory (Variables|/Game/InDevelop/UI/Main.Main_C|GetInventory _main))
  ;[1 1 1] Eating
  (:Pressed
    (if (not (Variables|Food|GetisBuffActive))
      (switch int (Utilities|Array|Get(acopy) (Variables|Inventory|GetInventory) (Variables|Inventory|GetInventorySelect))
        (:1
          (bind _output_get (Variables|Food|SetFoodBuff 1))
          (CallFunction|Food _output_get))
        (:2
          (bind _output_get_2 (Variables|Food|SetFoodBuff 2))
          (CallFunction|Food _output_get_2))
        (:3
          (bind _output_get_3 (Variables|Food|SetFoodBuff 3))
          (CallFunction|Food _output_get_3))
        (:4
          (bind _output_get_4 (Variables|Food|SetFoodBuff 4))
          (CallFunction|Food _output_get_4)))
      (Utilities|Array|SetArrayElem (Variables|Inventory|GetInventory) _inventoryselect 0)
      (Utilities|FlowControl|Sequence
        (:then_0
          ;[1 1 1] Inventory Show
          (Utilities|FlowControl|Sequence
            (:then_0
              (switch int (Utilities|Array|Length (Variables|Inventory|GetInventory))
                (:1
                  (Widget|SetVisibility _inventory "Visible"))
                (:2
                  (Widget|SetVisibility _inventory "Visible"))
                (:3
                  (Widget|SetVisibility _inventory "Visible")))
              (Utilities|FlowControl|Delay 3.0)
              (Widget|SetVisibility (Variables|/Game/InDevelop/UI/Main.Main_C|GetInventory (Variables|UI|GetMain)) "Hidden"))))
        (:then_1
          (Default|ChangeImageonArray (Variables|UI|GetMain) _inventoryselect 0 (Variables|Inventory|GetInventorySelect)))))))

(event Input|KeyboardEvents|C
  (params (Key :type Key%20Structure :default "None"))
  (:Pressed
    (for _array_element (Variables|Inventory|GetInventory)
      (Development|PrintString (Utilities|String|ToString(Integer) _array_element))
      (Development|PrintString (Utilities|String|ToString(Boolean) (Variables|Inventory|GetisInventoryAvailable))))))

(event Input|KeyboardEvents|NumPadTwo
  (params (Key :type Key%20Structure :default "None"))
  (bind _main (Variables|UI|GetMain))
  ;[1 1 1] DevThings
  ;;[1 1 1] Dev Jump
  (:Pressed
    (Default|Num2 _main)
    (switch Utilities|FlowControl|Switch|SwitchonECheckBoxState (Class|CheckBox|GetCheckedState (Variables|/Game/InDevelop/UI/Main.Main_C|Getwb_jump _main))
      (:Unchecked
        (Variables|Dev|Setwb_jump false))
      (:Checked
        (Variables|Dev|Setwb_jump true)))))

(event Input|MouseEvents|MiddleMouseButton
  (params (Key :type Key%20Structure :default "None")))

(event Input|MouseEvents|LeftMouseButton
  (params (Key :type Key%20Structure :default "None"))
  (bind _pixelperfectcamera (Variables|Components|GetPixelPerfectCamera))
  (bind _returnvalue (Transformation|GetWorldLocation _pixelperfectcamera))
  ;[1 1 1] Holding and rotating object
  (:Pressed
    (bind (_outhit _returnvalue_2) (Collision|LineTraceByChannel _returnvalue (+ (* (Math|Vector|GetForwardVector _pixelperfectcamera) (Variables|Pickup|GetPickupDIstance)) _returnvalue) "TraceTypeQuery1" false 0 "None"))
    (if _returnvalue_2
      (if (Physics|IsSimulatingPhysics (Variables|/Script/Engine.Actor|GetRootComponent (.HitActor (Collision|BreakHitResult _outhit))) "None")
        (bind _output_get (Variables|Default|SetCurrentlyHeldItem (.HitComponent (Collision|BreakHitResult _outhit))))
        (Class|PhysicsHandleComponent|GrabComponentatLocation (Variables|Default|GetPhysicsHandle) (.HitComponent (Collision|BreakHitResult _outhit)) "None" (Transformation|GetWorldLocation (.HitComponent (Collision|BreakHitResult _outhit))))
        (Variables|Pickup|SetisHoldingSmth true))))
  (:Released
    (Physics|Components|PhysicsHandle|ReleaseComponent (Variables|Default|GetPhysicsHandle))
    (Utilities|FlowControl|Sequence
      (:then_0
        (Variables|Pickup|SetisHoldingSmth false)
        (Variables|Pickup|SetheldObgectRotation 0.0)
        (Widget|SetVisibility (Variables|/Game/InDevelop/UI/Main.Main_C|GetAxisXBorder (Variables|UI|GetMain)) "Hidden")))))

(event Input|MouseEvents|MouseWheelUp
  (params (Key :type Key%20Structure :default "None"))
  (bind _main (Variables|UI|GetMain))
  (bind _inventory (Variables|/Game/InDevelop/UI/Main.Main_C|GetInventory _main))
  ;[1 1 1] Inventory Select
  (:Pressed
    (Variables|Inventory|SetInventorySelect (+ (Variables|Inventory|GetInventorySelect) 1))
    (if (> (Variables|Inventory|GetInventorySelect) 2)
      (Variables|Inventory|SetInventorySelect 0))
    (Default|SelectOverlay (Variables|UI|GetMain) (Variables|Inventory|GetInventorySelect))
    ;[1 1 1] Inventory Show
    (Utilities|FlowControl|Sequence
      (:then_0
        (switch int (Utilities|Array|Length (Variables|Inventory|GetInventory))
          (:1
            (Widget|SetVisibility _inventory "Visible"))
          (:2
            (Widget|SetVisibility _inventory "Visible"))
          (:3
            (Widget|SetVisibility _inventory "Visible")))
        (Utilities|FlowControl|Delay 3.0)
        (Widget|SetVisibility (Variables|/Game/InDevelop/UI/Main.Main_C|GetInventory (Variables|UI|GetMain)) "Hidden")))))

(event Input|MouseEvents|MouseWheelDown
  (params (Key :type Key%20Structure :default "None"))
  (bind _main (Variables|UI|GetMain))
  (bind _inventory (Variables|/Game/InDevelop/UI/Main.Main_C|GetInventory _main))
  ;[1 1 1] Inventory Select
  (:Pressed
    (Variables|Inventory|SetInventorySelect (- (Variables|Inventory|GetInventorySelect) 1))
    (if (< (Variables|Inventory|GetInventorySelect) 0)
      (Variables|Inventory|SetInventorySelect 2))
    (Default|SelectOverlay (Variables|UI|GetMain) (Variables|Inventory|GetInventorySelect))
    ;[1 1 1] Inventory Show
    (Utilities|FlowControl|Sequence
      (:then_0
        (switch int (Utilities|Array|Length (Variables|Inventory|GetInventory))
          (:1
            (Widget|SetVisibility _inventory "Visible"))
          (:2
            (Widget|SetVisibility _inventory "Visible"))
          (:3
            (Widget|SetVisibility _inventory "Visible")))
        (Utilities|FlowControl|Delay 3.0)
        (Widget|SetVisibility (Variables|/Game/InDevelop/UI/Main.Main_C|GetInventory (Variables|UI|GetMain)) "Hidden")))))

(event Input|KeyboardEvents|R
  (params (Key :type Key%20Structure :default "None"))
  ;[1 1 1] Holding and rotating object
  (:Pressed
    (Utilities|FlowControl|Sequence
      (:then_0
        (if (== (Variables|Pickup|GetholdingObjectRotation) 0)
          (Variables|Pickup|SetholdingObjectRotation 1)
          (elif (== (Variables|Pickup|GetholdingObjectRotation) 1)
            (Variables|Pickup|SetholdingObjectRotation 2)
            (else
              (Variables|Pickup|SetholdingObjectRotation 0)))))
      (:then_1
        (Widget|SetVisibility (Variables|/Game/InDevelop/UI/Main.Main_C|GetAxisXBorder (Variables|UI|GetMain)) "Hidden")))))

(event Input|KeyboardEvents|F
  (params (Key :type Key%20Structure :default "None"))
  (bind (_free_index _isfree) (CallFunction|FindFreeSpaceinInventory))
  (bind _main (Variables|UI|GetMain))
  (bind _pixelperfectcamera (Variables|Components|GetPixelPerfectCamera))
  (bind _returnvalue (Transformation|GetWorldLocation _pixelperfectcamera))
  (bind _inventory (Variables|/Game/InDevelop/UI/Main.Main_C|GetInventory _main))
  ;[1 1 1] Add Object to Inventory
  (:Pressed
    (bind (_outhit _returnvalue_2) (Collision|LineTraceByChannel _returnvalue (+ (* (Math|Vector|GetForwardVector _pixelperfectcamera) (Variables|Pickup|GetPickupDIstance)) _returnvalue) "TraceTypeQuery1" false 0 "None"))
    (if _returnvalue_2
      (if (Physics|IsSimulatingPhysics (Variables|/Script/Engine.Actor|GetRootComponent (.HitActor (Collision|BreakHitResult _outhit))) "None")
        (for _array_element (Variables|/Script/Engine.Actor|GetTags (.HitActor (Collision|BreakHitResult _outhit)))
          (if (Variables|Inventory|GetisInventoryAvailable)
            (if _isfree
              (Utilities|Array|SetArrayElem (Variables|Inventory|GetInventory) _free_index (Math|Conversions|ToInteger(Byte) (Utilities|String|ToString(Name) _array_element)))
              (Default|ChangeImageonArray (Variables|UI|GetMain) _free_index (Math|Conversions|ToInteger(Byte) (Utilities|String|ToString(Name) _array_element)) (Variables|Inventory|GetInventorySelect))
              (Utilities|FlowControl|Sequence
                (:then_0
                  (if (== _free_index 2)
                    (Development|PrintText "Inv not available")
                    (else
                      (Variables|Inventory|SetisInventoryAvailable true)
                      (Development|PrintText "Inv available"))))
                (:then_1
                  ;[1 1 1] Inventory Show
                  (switch int (Utilities|Array|Length (Variables|Inventory|GetInventory))
                    (:1
                      (Widget|SetVisibility _inventory "Visible"))
                    (:2
                      (Widget|SetVisibility _inventory "Visible"))
                    (:3
                      (Widget|SetVisibility _inventory "Visible")))
                  (Utilities|FlowControl|Delay 3.0)
                  (Widget|SetVisibility (Variables|/Game/InDevelop/UI/Main.Main_C|GetInventory (Variables|UI|GetMain)) "Hidden")))
              (else
                (Development|PrintText "Maximum Inventory Space Reached" :!label _label)))
            (else
              (goto _label))))))))

(event Input|KeyboardEvents|E
  (params (Key :type Key%20Structure :default "None"))
  (bind _main (Variables|UI|GetMain))
  (bind _inventory (Variables|/Game/InDevelop/UI/Main.Main_C|GetInventory _main))
  ;[1 1 1] Inventory Show
  (:Pressed
    (Utilities|FlowControl|Sequence
      (:then_0
        (switch int (Utilities|Array|Length (Variables|Inventory|GetInventory))
          (:1
            (Widget|SetVisibility _inventory "Visible"))
          (:2
            (Widget|SetVisibility _inventory "Visible"))
          (:3
            (Widget|SetVisibility _inventory "Visible")))
        (Utilities|FlowControl|Delay 3.0)
        (Widget|SetVisibility (Variables|/Game/InDevelop/UI/Main.Main_C|GetInventory (Variables|UI|GetMain)) "Hidden")))))

(fn ConstructionScript)

(fn StartSprint
  (Variables|/Script/Engine.CharacterMovementComponent|SetMaxWalkSpeed (Variables|Character|GetCharacterMovement) (Variables|Moving|GetsprintSpeed))
  (Variables|Moving|SetIsSprint true)
  (Development|PrintText "Sprinting"))

(fn StopSprint
  (Variables|/Script/Engine.CharacterMovementComponent|SetMaxWalkSpeed (Variables|Character|GetCharacterMovement) (Variables|Moving|GetbaseSpeed))
  (Variables|Moving|SetIsSprint false)
  (Development|PrintText "NotSprinting"))

(fn DevMenuon
  (Widget|SetVisibility (Variables|/Game/InDevelop/UI/Main.Main_C|GetDevMenu_Widget (Variables|UI|GetMain)) "Visible"))

(fn DevMenuOff
  (Widget|SetVisibility (Variables|/Game/InDevelop/UI/Main.Main_C|GetDevMenu_Widget (Variables|UI|GetMain)) "Hidden"))

(fn FindFreeSpaceinInventory
  (for (_array_element _array_index) (Variables|Inventory|GetInventory)
    (switch int _array_index
      (:0
        (if (== _array_element 0)
          (if (Variables|Inventory|GetisInventoryAvailable)
            (Development|PrintString "1 is zero")
            (Variables|Inventory|SetisInventoryAvailable false)
            (return 0 true))
          (else
            (Development|PrintString "1 is full"))))
      (:1
        (if (== _array_element 0)
          (if (Variables|Inventory|GetisInventoryAvailable)
            (Development|PrintString "2 is zero")
            (Variables|Inventory|SetisInventoryAvailable false)
            (return 1 true))
          (else
            (Development|PrintString "2 is full"))))
      (:2
        (if (== _array_element 0)
          (if (Variables|Inventory|GetisInventoryAvailable)
            (Development|PrintString "3 is zero")
            (Variables|Inventory|SetisInventoryAvailable false)
            (return 2 true))
          (else
            (Development|PrintString "3 is full")))))))