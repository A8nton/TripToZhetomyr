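; Background tile manager that keeps spawning BP_BackgroundTile actors relative to the player's X position.
; On BeginPlay it spawns the first tile at the player's X plus TileOffset and stores it as the last spawned tile.
; Each Tick it spawns and stores another whenever the player is within a fixed X distance of that last tile.
; It never destroys tiles itself.
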(event EventBeginPlay
  (bind _returnvalue (Game|SpawnActorfromClass "/Game/InDevelop/Blueprints/Meshes/Nature/BP_BackgroundTile.BP_BackgroundTile_C" (Math|Conversions|ToTransform(Vector) (+ (Math|Vector|MakeVector (.x (Transformation|GetActorLocation (Game|GetPlayerCharacter 0))) 0.0 0.0) (Variables|Default|GetTileOffset))) "Undefined" "MultiplyWithRoot" 0 0))
  (Variables|Default|SetlastSpawnedTile _returnvalue)
  (Variables|Default|SetisSpawnedFirst true))

(event EventTick
  (params (DeltaSeconds :type Float%20%28single-precision%29))
  (if (Variables|Default|GetisSpawnedFirst)
    (if (<= (Math|Vector|Distance(Vector) (Math|Vector|MakeVector (.x (Transformation|GetActorLocation (Variables|Default|GetlastSpawnedTile))) 0.0 0.0) (Math|Vector|MakeVector (.x (Transformation|GetActorLocation (Game|GetPlayerCharacter 0))) 0.0 0.0)) 3.8e+03)
      (bind _returnvalue (Game|SpawnActorfromClass "/Game/InDevelop/Blueprints/Meshes/Nature/BP_BackgroundTile.BP_BackgroundTile_C" (Math|Conversions|ToTransform(Vector) (+ (Math|Vector|MakeVector (.x (Transformation|GetActorLocation (Game|GetPlayerCharacter 0))) 0.0 0.0) (Variables|Default|GetTileOffset))) "Undefined" "MultiplyWithRoot" 0 0))
      (Variables|Default|SetlastSpawnedTile _returnvalue))))

(fn ConstructionScript)