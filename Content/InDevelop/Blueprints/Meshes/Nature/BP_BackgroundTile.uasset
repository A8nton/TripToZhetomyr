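; BP_BackgroundTile is a background scenery tile actor that moves along the world X axis.
; Every Tick it offsets its position by MoveSpeed scaled by delta time, so movement is frame-rate independent.
; It then measures its distance to the player character and destroys itself once beyond a fixed cutoff.
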(event EventTick
  (params (DeltaSeconds :type Float%20%28single-precision%29))
  (Utilities|FlowControl|Sequence
    (:then_0
      (Transformation|AddActorWorldOffset (Math|Vector|MakeVector (* (Variables|Default|GetmoveSpeed) DeltaSeconds) 0.0 0.0))
      (if (> (Math|Vector|Distance(Vector) (Transformation|GetActorLocation self) (Transformation|GetActorLocation (Game|GetPlayerCharacter 0))) 6e+03)
        (Actor|DestroyActor)))))

(fn ConstructionScript)