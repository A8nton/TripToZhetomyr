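; BP_TrainDoorEntr is a train entrance door that slides open on trigger overlap and may set up a puzzle.
; On BeginPlay, a one-in-five roll spawns BP_Simon at the PuzzleSpawn-tagged component and destroys BP_Monster.
; Overlap plays the Opening timeline to drive the door's world Y, then disables the trigger's collision.
; A separate doorclose event moves the door through a Closing timeline.
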(event OnComponentBeginOverlap(InteractionTrigger)
  (params (OverlappedComponent :type Primitive%20Component%20Object%20Reference) (OtherActor :type Actor%20Object%20Reference) (OtherComp :type Primitive%20Component%20Object%20Reference) (OtherBodyIndex :type Integer) (bFromSweep :type Boolean) (SweepResult :type Hit%20Result%20Structure%20%28by%20ref%29))
  (bind _door (Variables|Default|GetDoor))
  (bind _returnvalue (Transformation|GetWorldLocation _door))
  (if (Utilities|IsValid (Variables|Default|GetInteractionTrigger))
    (bind _dooropen (Timeline|Opening PlayFromStart)
      (:Update
        (Transformation|SetWorldLocation _door (Math|Vector|MakeVector (.x _returnvalue) _dooropen (.z _returnvalue)) false false))
      (:Finished
        (CallFunction|DisableDoor)))))

(event Custom|doorclose
  (bind _door (Variables|Default|GetDoor))
  (bind _returnvalue (Transformation|GetWorldLocation _door))
  (Timeline|closing PlayFromStart
    (:Update
      (Transformation|SetWorldLocation _door (Math|Vector|MakeVector (+ (.x _returnvalue) 2.0) 0.0 (.z _returnvalue)) false false))))

(event EventBeginPlay
  (switch int (Math|Random|RandomIntegerinRange 0 4)
    (:1
      (bind _asscene_component (Utilities|Casting|CastToSceneComponent (Utilities|Array|Get(acopy) (Actor|GetComponentsbyTag "/Script/Engine.ActorComponent" "PuzzleSpawn"))))
      (bind _returnvalue (Game|SpawnActorfromClass "/Game/InDevelop/Blueprints/Puzzles/SimonSays/BP_Simon.BP_Simon_C" (Math|Conversions|ToTransform(Vector) (Transformation|GetWorldLocation _asscene_component)) "AlwaysSpawn" "MultiplyWithRoot" 0 0))
      (bind _returnvalue_2 (Actor|GetActorOfClass "/Game/InDevelop/Blueprints/BP_Monster.BP_Monster_C"))
      (Actor|DestroyActor _returnvalue_2))))

(fn ConstructionScript)

(fn DisableDoor
  (Collision|SetCollisionEnabled (Variables|Default|GetInteractionTrigger) "NoCollision"))