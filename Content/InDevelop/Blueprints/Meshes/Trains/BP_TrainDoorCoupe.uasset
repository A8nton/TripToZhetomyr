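; Train compartment door Blueprint with four doors that open when their trigger volumes are overlapped and close automatically.
; Each overlap plays an open timeline driving that door's absolute world Z, then after a delay sets a closing flag.
; Tick polls the flags to play close timelines, which re-enable the trigger when finished.
; Overlaps disable trigger collision, but the second door's overlap disables the third door's trigger instead of its own.
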(event OnComponentBeginOverlap(InteractionTrigger)
  (params (OverlappedComponent :type Primitive%20Component%20Object%20Reference) (OtherActor :type Actor%20Object%20Reference) (OtherComp :type Primitive%20Component%20Object%20Reference) (OtherBodyIndex :type Integer) (bFromSweep :type Boolean) (SweepResult :type Hit%20Result%20Structure%20%28by%20ref%29))
  (bind _door (Variables|Default|GetDoor))
  (bind _returnvalue (Transformation|GetWorldLocation _door))
  (CallFunction|DisableDoor1)
  (bind _coupeopen (Timeline|doorOpen PlayFromStart)
    (:Update
      (Transformation|SetWorldLocation _door (Math|Vector|MakeVector (.x _returnvalue) (.y _returnvalue) _coupeopen) false false))
    (:Finished
      (Utilities|FlowControl|Delay 3.0)
      (Variables|Default|SetisDoor1Closing true))))

(event OnComponentBeginOverlap(InteractionTrigger1)
  (params (OverlappedComponent :type Primitive%20Component%20Object%20Reference) (OtherActor :type Actor%20Object%20Reference) (OtherComp :type Primitive%20Component%20Object%20Reference) (OtherBodyIndex :type Integer) (bFromSweep :type Boolean) (SweepResult :type Hit%20Result%20Structure%20%28by%20ref%29))
  (bind _door1 (Variables|Default|GetDoor1))
  (bind _returnvalue (Transformation|GetWorldLocation _door1))
  (CallFunction|DisableDoor3)
  (bind _coupeopen (Timeline|Timeline PlayFromStart)
    (:Update
      (Transformation|SetWorldLocation _door1 (Math|Vector|MakeVector (.x _returnvalue) (.y _returnvalue) _coupeopen) false false))
    (:Finished
      (Utilities|FlowControl|Delay 3.0)
      (Variables|Default|SetisDoor2Closing true))))

(event OnComponentBeginOverlap(InteractionTrigger2)
  (params (OverlappedComponent :type Primitive%20Component%20Object%20Reference) (OtherActor :type Actor%20Object%20Reference) (OtherComp :type Primitive%20Component%20Object%20Reference) (OtherBodyIndex :type Integer) (bFromSweep :type Boolean) (SweepResult :type Hit%20Result%20Structure%20%28by%20ref%29))
  (bind _door2 (Variables|Default|GetDoor2))
  (bind _returnvalue (Transformation|GetWorldLocation _door2))
  (CallFunction|DisableDoor3)
  (bind _coupeopen (Timeline|Timeline_0 PlayFromStart)
    (:Update
      (Transformation|SetWorldLocation _door2 (Math|Vector|MakeVector (.x _returnvalue) (.y _returnvalue) _coupeopen) false false))
    (:Finished
      (Utilities|FlowControl|Delay 3.0)
      (Variables|Default|SetisDoor3Closing true))))

(event OnComponentBeginOverlap(InteractionTrigger3)
  (params (OverlappedComponent :type Primitive%20Component%20Object%20Reference) (OtherActor :type Actor%20Object%20Reference) (OtherComp :type Primitive%20Component%20Object%20Reference) (OtherBodyIndex :type Integer) (bFromSweep :type Boolean) (SweepResult :type Hit%20Result%20Structure%20%28by%20ref%29))
  (bind _door3 (Variables|Default|GetDoor3))
  (bind _returnvalue (Transformation|GetWorldLocation _door3))
  (CallFunction|DisableDoor4)
  (bind _coupeopen (Timeline|Timeline_1 PlayFromStart)
    (:Update
      (Transformation|SetWorldLocation _door3 (Math|Vector|MakeVector (.x _returnvalue) (.y _returnvalue) _coupeopen) false false))
    (:Finished
      (Utilities|FlowControl|Delay 3.0)
      (Variables|Default|SetisDoor4Closing true))))

(event EventTick
  (params (DeltaSeconds :type Float%20%28single-precision%29))
  (bind _door3 (Variables|Default|GetDoor3))
  (bind _door2 (Variables|Default|GetDoor2))
  (bind _door1 (Variables|Default|GetDoor1))
  (bind _door (Variables|Default|GetDoor))
  (bind _returnvalue (Transformation|GetWorldLocation _door3))
  (bind _returnvalue_2 (Transformation|GetWorldLocation _door))
  (bind _returnvalue_3 (Transformation|GetWorldLocation _door1))
  (bind _returnvalue_4 (Transformation|GetWorldLocation _door2))
  (Utilities|FlowControl|Sequence
    (:then_0
      (if (Variables|Default|GetisDoor1Closing)
        (Variables|Default|SetisDoor1Closing false)
        (bind _coupeclose (Timeline|doorClose PlayFromStart)
          (:Update
            (Transformation|SetWorldLocation _door (Math|Vector|MakeVector (.x _returnvalue_2) (.y _returnvalue_2) _coupeclose) false false))
          (:Finished
            (CallFunction|EnableDoor1)))))
    (:then_1
      (if (Variables|Default|GetisDoor2Closing)
        (Variables|Default|SetisDoor2Closing false)
        (bind _coupeclose_2 (Timeline|Timeline_2 PlayFromStart)
          (:Update
            (Transformation|SetWorldLocation _door1 (Math|Vector|MakeVector (.x _returnvalue_3) (.y _returnvalue_3) _coupeclose_2) false false))
          (:Finished
            (CallFunction|EnableDoor2)))))
    (:then_2
      (if (Variables|Default|GetisDoor3Closing)
        (Variables|Default|SetisDoor3Closing false)
        (bind _coupeclose_3 (Timeline|Timeline_3 PlayFromStart)
          (:Update
            (Transformation|SetWorldLocation _door2 (Math|Vector|MakeVector (.x _returnvalue_4) (.y _returnvalue_4) _coupeclose_3) false false))
          (:Finished
            (CallFunction|EnableDoor3)))))
    (:then_3
      (if (Variables|Default|GetisDoor4Closing)
        (Variables|Default|SetisDoor4Closing false)
        (bind _coupeclose_4 (Timeline|Timeline_4 PlayFromStart)
          (:Update
            (Transformation|SetWorldLocation _door3 (Math|Vector|MakeVector (.x _returnvalue) (.y _returnvalue) _coupeclose_4) false false))
          (:Finished
            (CallFunction|EnableDoor4)))))))

(fn ConstructionScript)

(fn EnableDoor1
  (Collision|SetCollisionEnabled (Variables|Default|GetInteractionTrigger) "QueryOnly"))

(fn DisableDoor1
  (Collision|SetCollisionEnabled (Variables|Default|GetInteractionTrigger) "NoCollision"))

(fn EnableDoor2
  (Collision|SetCollisionEnabled (Variables|Default|GetInteractionTrigger1) "QueryOnly"))

(fn EnableDoor3
  (Collision|SetCollisionEnabled (Variables|Default|GetInteractionTrigger2) "QueryOnly"))

(fn EnableDoor4
  (Collision|SetCollisionEnabled (Variables|Default|GetInteractionTrigger3) "QueryOnly"))

(fn DisableDoor2
  (Collision|SetCollisionEnabled (Variables|Default|GetInteractionTrigger1) "NoCollision"))

(fn DisableDoor3
  (Collision|SetCollisionEnabled (Variables|Default|GetInteractionTrigger2) "NoCollision"))

(fn DisableDoor4
  (Collision|SetCollisionEnabled (Variables|Default|GetInteractionTrigger3) "NoCollision"))