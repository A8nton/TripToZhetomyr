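; Train coupe car actor that randomly dresses itself with props and event triggers when play begins.
; BeginPlay notifies the navigation system, then rolls per tagged scene component to spawn props from the PropsU and PropsN arrays.
; A further roll may spawn BP_trigger, or BP_RunningMonsterTrigger if BP_Monster's Spawned flag is false, at tagged components.
; The Puzzleremover overlap destroys actors whose root component is tagged "simon".
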(event OnComponentBeginOverlap(puzzleremover)
  (params (OverlappedComponent :type Primitive%20Component%20Object%20Reference) (OtherActor :type Actor%20Object%20Reference) (OtherComp :type Primitive%20Component%20Object%20Reference) (OtherBodyIndex :type Integer) (bFromSweep :type Boolean) (SweepResult :type Hit%20Result%20Structure%20%28by%20ref%29))
  (if (Components|ComponentHasTag (Variables|/Script/Engine.Actor|GetRootComponent OtherActor) "simon")
    (Actor|DestroyActor OtherActor)
    (Development|PrintString "destroyes")))

(event EventBeginPlay
  (bind _returnvalue (Math|Random|RandomIntegerinRange 0 1))
  (bind _returnvalue_2 (Math|Random|RandomIntegerinRange 0 3))
  (bind _returnvalue_3 (Math|Random|RandomIntegerinRange 0 2))
  (bind _returnvalue_4 (Math|Random|RandomIntegerinRange 0 3))
  (bind _propsu (Variables|Default|GetPropsU))
  (bind _propsn (Variables|Default|GetPropsN))
  (bind _output (Utilities|Array|Get(acopy) _propsn _returnvalue_4))
  (bind _output_2 (Utilities|Array|Get(acopy) _propsu _returnvalue_2))
  (bind _returnvalue_5 (== _returnvalue_3 1))
  (bind _returnvalue_6 (== _returnvalue 1))
  (Utilities|FlowControl|Sequence
    (:then_0
      (Class|NavigationSystemV1|OnNavigationBoundsUpdated (Class|NavigationSystemV1|GetNavigationSystem))
      (Utilities|FlowControl|Sequence
        (:then_0
          (Utilities|FlowControl|Sequence
            (:then_0
              (bind _asscene_component (Utilities|Casting|CastToSceneComponent (Utilities|Array|Get(acopy) (Actor|GetComponentsbyTag "/Script/Engine.ActorComponent" "Pr_U1"))))
              (if _returnvalue_5
                (Game|SpawnActorfromClass _output_2 (Math|Conversions|ToTransform(Vector) (Transformation|GetWorldLocation _asscene_component)) "Undefined" "MultiplyWithRoot" 0 0)))
            (:then_1
              (bind _asscene_component_2 (Utilities|Casting|CastToSceneComponent (Utilities|Array|Get(acopy) (Actor|GetComponentsbyTag "/Script/Engine.ActorComponent" "Pr_U2"))))
              (if _returnvalue_5
                (Game|SpawnActorfromClass _output_2 (Math|Conversions|ToTransform(Vector) (Transformation|GetWorldLocation _asscene_component_2)) "Undefined" "MultiplyWithRoot" 0 0)))
            (:then_2
              (bind _asscene_component_3 (Utilities|Casting|CastToSceneComponent (Utilities|Array|Get(acopy) (Actor|GetComponentsbyTag "/Script/Engine.ActorComponent" "Pr_U3"))))
              (if _returnvalue_5
                (Game|SpawnActorfromClass _output_2 (Math|Conversions|ToTransform(Vector) (Transformation|GetWorldLocation _asscene_component_3)) "Undefined" "MultiplyWithRoot" 0 0)))
            (:then_3
              (bind _asscene_component_4 (Utilities|Casting|CastToSceneComponent (Utilities|Array|Get(acopy) (Actor|GetComponentsbyTag "/Script/Engine.ActorComponent" "Pr_U4"))))
              (if _returnvalue_5
                (Game|SpawnActorfromClass _output_2 (Math|Conversions|ToTransform(Vector) (Transformation|GetWorldLocation _asscene_component_4)) "Undefined" "MultiplyWithRoot" 0 0)))
            (:then_4
              (bind _asscene_component_5 (Utilities|Casting|CastToSceneComponent (Utilities|Array|Get(acopy) (Actor|GetComponentsbyTag "/Script/Engine.ActorComponent" "Pr_U5"))))
              (if _returnvalue_5
                (Game|SpawnActorfromClass _output_2 (Math|Conversions|ToTransform(Vector) (Transformation|GetWorldLocation _asscene_component_5)) "Undefined" "MultiplyWithRoot" 0 0)))
            (:then_5
              (bind _asscene_component_6 (Utilities|Casting|CastToSceneComponent (Utilities|Array|Get(acopy) (Actor|GetComponentsbyTag "/Script/Engine.ActorComponent" "Pr_U6"))))
              (if _returnvalue_5
                (Game|SpawnActorfromClass _output_2 (Math|Conversions|ToTransform(Vector) (Transformation|GetWorldLocation _asscene_component_6)) "Undefined" "MultiplyWithRoot" 0 0)))
            (:then_6
              (Utilities|FlowControl|Sequence
                (:then_0
                  (if _returnvalue_5
                    (if (not (Variables|Default|GetbisCreatingtrigger))
                      (Utilities|FlowControl|DoN 1
                        (:Exit
                          (CallFunction|CreatingTrigger))))
                    (elif (not (Variables|Default|GetbisCreatingtrigger))
                      (if (== (Math|Random|RandomIntegerinRange 0 2) 0)
                        (bind _returnvalue_7 (Actor|GetActorOfClass "/Game/InDevelop/Blueprints/BP_Monster.BP_Monster_C"))
                        (if (not (Variables|/Game/InDevelop/Blueprints/BP_Monster.BP_Monster_C|GetSpawned _returnvalue_7))
                          (CallFunction|CreateMonsterTrigger)
                          (Variables|Default|SetbisCreatingtrigger true))))))))))
        (:then_1
          (Utilities|FlowControl|Sequence
            (:then_0
              (bind _asscene_component_7 (Utilities|Casting|CastToSceneComponent (Utilities|Array|Get(acopy) (Actor|GetComponentsbyTag "/Script/Engine.ActorComponent" "Pr_N1"))))
              (if _returnvalue_6
                (Game|SpawnActorfromClass _output (Math|Conversions|ToTransform(Vector) (Transformation|GetWorldLocation _asscene_component_7)) "Undefined" "MultiplyWithRoot" 0 0)))
            (:then_1
              (bind _asscene_component_8 (Utilities|Casting|CastToSceneComponent (Utilities|Array|Get(acopy) (Actor|GetComponentsbyTag "/Script/Engine.ActorComponent" "Pr_N2"))))
              (if _returnvalue_6
                (Game|SpawnActorfromClass _output (Math|Conversions|ToTransform(Vector) (Transformation|GetWorldLocation _asscene_component_8)) "Undefined" "MultiplyWithRoot" 0 0)))
            (:then_2
              (bind _asscene_component_9 (Utilities|Casting|CastToSceneComponent (Utilities|Array|Get(acopy) (Actor|GetComponentsbyTag "/Script/Engine.ActorComponent" "Pr_N3"))))
              (if _returnvalue_6
                (Game|SpawnActorfromClass _output (Math|Conversions|ToTransform(Vector) (Transformation|GetWorldLocation _asscene_component_9)) "Undefined" "MultiplyWithRoot" 0 0)))
            (:then_3
              (bind _asscene_component_10 (Utilities|Casting|CastToSceneComponent (Utilities|Array|Get(acopy) (Actor|GetComponentsbyTag "/Script/Engine.ActorComponent" "Pr_N4"))))
              (if _returnvalue_6
                (Game|SpawnActorfromClass _output (Math|Conversions|ToTransform(Vector) (Transformation|GetWorldLocation _asscene_component_10)) "Undefined" "MultiplyWithRoot" 0 0)))))))))

(fn ConstructionScript)

(fn SpawnNavMesh
  (Transformation|SetActorLocation (Variables|Default|GetNavMeshVolume) (Transformation|GetWorldLocation (Utilities|Array|Get(acopy) (Actor|GetComponentsbyTag "/Script/Engine.SceneComponent" "NavMesh"))) false true))

(fn CreatingTrigger
  (bind _asscene_component (Utilities|Casting|CastToSceneComponent (Utilities|Array|Get(acopy) (Actor|GetComponentsbyTag "/Script/Engine.ActorComponent" "Trigger"))))
  (Utilities|FlowControl|DoN 1
    (:Exit
      (bind _returnvalue (Game|SpawnActorfromClass "/Game/InDevelop/Blueprints/BP_trigger.BP_trigger_C" (Math|Transform|MakeTransform (Transformation|GetWorldLocation _asscene_component) (Transformation|GetWorldRotation _asscene_component)) "AlwaysSpawn" "MultiplyWithRoot" 0 0))
      (Variables|Default|SetbisCreatingtrigger true)
      (Development|PrintString (Utilities|GetDisplayName _returnvalue)))))

(fn CreateMonsterTrigger
  (bind _returnvalue (Actor|GetComponentsbyTag "/Script/Engine.SceneComponent" "MonsterTrigger"))
  (bind _output (Utilities|Array|Get(acopy) _returnvalue))
  (Game|SpawnActorfromClass "/Game/InDevelop/Blueprints/BP_RunningMonsterTrigger.BP_RunningMonsterTrigger_C" (Math|Transform|MakeTransform (Transformation|GetWorldLocation _output) (Transformation|GetWorldRotation _output)) "AlwaysSpawn" "MultiplyWithRoot" 0 0))