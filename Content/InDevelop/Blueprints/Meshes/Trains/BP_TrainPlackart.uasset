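; Platzkart train car actor that randomly dresses itself with props and may set up a monster encounter on BeginPlay.
; Scene components tagged Pr_U and Pr_N mark prop slots, each rolling a chance to spawn a random class from PropsU or PropsN.
; If a BP_Monster exists and is not yet Spawned, a coin flip calls SpawnMonster, which places a BP_MonsterSpawnTrigger at the tagged MonsterTriggerPlackart component.
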(event EventBeginPlay
  (bind _returnvalue (Math|Random|RandomIntegerinRange 0 3))
  (bind _returnvalue_2 (Math|Random|RandomIntegerinRange 0 3))
  (bind _returnvalue_3 (Math|Random|RandomIntegerinRange 0 3))
  (bind _returnvalue_4 (Math|Random|RandomIntegerinRange 0 2))
  (bind _propsu (Variables|Default|GetPropsU))
  (bind _propsn (Variables|Default|GetPropsN))
  (bind _output (Utilities|Array|Get(acopy) _propsn _returnvalue_3))
  (bind _output_2 (Utilities|Array|Get(acopy) _propsu _returnvalue_2))
  (bind _returnvalue_5 (== _returnvalue 1))
  (bind _returnvalue_6 (== _returnvalue_4 1))
  (Utilities|FlowControl|Sequence
    (:then_0
      (Utilities|FlowControl|Sequence
        (:then_0
          (bind _asscene_component (Utilities|Casting|CastToSceneComponent (Utilities|Array|Get(acopy) (Actor|GetComponentsbyTag "/Script/Engine.ActorComponent" "Pr_U1"))))
          (if _returnvalue_6
            (Game|SpawnActorfromClass _output_2 (Math|Conversions|ToTransform(Vector) (Transformation|GetWorldLocation _asscene_component)) "Undefined" "MultiplyWithRoot" 0 0)))
        (:then_1
          (bind _asscene_component_2 (Utilities|Casting|CastToSceneComponent (Utilities|Array|Get(acopy) (Actor|GetComponentsbyTag "/Script/Engine.ActorComponent" "Pr_U2"))))
          (if _returnvalue_6
            (Game|SpawnActorfromClass _output_2 (Math|Conversions|ToTransform(Vector) (Transformation|GetWorldLocation _asscene_component_2)) "Undefined" "MultiplyWithRoot" 0 0)))
        (:then_2
          (bind _asscene_component_3 (Utilities|Casting|CastToSceneComponent (Utilities|Array|Get(acopy) (Actor|GetComponentsbyTag "/Script/Engine.ActorComponent" "Pr_U3"))))
          (if _returnvalue_6
            (Game|SpawnActorfromClass _output_2 (Math|Conversions|ToTransform(Vector) (Transformation|GetWorldLocation _asscene_component_3)) "Undefined" "MultiplyWithRoot" 0 0)))
        (:then_3
          (bind _asscene_component_4 (Utilities|Casting|CastToSceneComponent (Utilities|Array|Get(acopy) (Actor|GetComponentsbyTag "/Script/Engine.ActorComponent" "Pr_U4"))))
          (if _returnvalue_6
            (Game|SpawnActorfromClass _output_2 (Math|Conversions|ToTransform(Vector) (Transformation|GetWorldLocation _asscene_component_4)) "Undefined" "MultiplyWithRoot" 0 0)))
        (:then_4
          (bind _asscene_component_5 (Utilities|Casting|CastToSceneComponent (Utilities|Array|Get(acopy) (Actor|GetComponentsbyTag "/Script/Engine.ActorComponent" "Pr_U5"))))
          (if _returnvalue_6
            (Game|SpawnActorfromClass _output_2 (Math|Conversions|ToTransform(Vector) (Transformation|GetWorldLocation _asscene_component_5)) "Undefined" "MultiplyWithRoot" 0 0)))
        (:then_5
          (bind _asscene_component_6 (Utilities|Casting|CastToSceneComponent (Utilities|Array|Get(acopy) (Actor|GetComponentsbyTag "/Script/Engine.ActorComponent" "Pr_U6"))))
          (if _returnvalue_6
            (Game|SpawnActorfromClass _output_2 (Math|Conversions|ToTransform(Vector) (Transformation|GetWorldLocation _asscene_component_6)) "Undefined" "MultiplyWithRoot" 0 0)))
        (:then_6
          (bind _returnvalue_7 (Actor|GetActorOfClass "/Game/InDevelop/Blueprints/BP_Monster.BP_Monster_C"))
          (if (Utilities|IsValid _returnvalue_7)
            (if (not (Variables|/Game/InDevelop/Blueprints/BP_Monster.BP_Monster_C|GetSpawned _returnvalue_7))
              (if (== (Math|Random|RandomIntegerinRange 0 1) 0)
                (CallFunction|SpawnMonster)))))))
    (:then_1
      (Utilities|FlowControl|Sequence
        (:then_0
          (bind _asscene_component_7 (Utilities|Casting|CastToSceneComponent (Utilities|Array|Get(acopy) (Actor|GetComponentsbyTag "/Script/Engine.ActorComponent" "Pr_N1"))))
          (if _returnvalue_5
            (Game|SpawnActorfromClass _output (Math|Conversions|ToTransform(Vector) (Transformation|GetWorldLocation _asscene_component_7)) "Undefined" "MultiplyWithRoot" 0 0)))
        (:then_1
          (bind _asscene_component_8 (Utilities|Casting|CastToSceneComponent (Utilities|Array|Get(acopy) (Actor|GetComponentsbyTag "/Script/Engine.ActorComponent" "Pr_N2"))))
          (if _returnvalue_5
            (Game|SpawnActorfromClass _output (Math|Conversions|ToTransform(Vector) (Transformation|GetWorldLocation _asscene_component_8)) "Undefined" "MultiplyWithRoot" 0 0)))
        (:then_2
          (bind _asscene_component_9 (Utilities|Casting|CastToSceneComponent (Utilities|Array|Get(acopy) (Actor|GetComponentsbyTag "/Script/Engine.ActorComponent" "Pr_N3"))))
          (if _returnvalue_5
            (Game|SpawnActorfromClass _output (Math|Conversions|ToTransform(Vector) (Transformation|GetWorldLocation _asscene_component_9)) "Undefined" "MultiplyWithRoot" 0 0)))
        (:then_3
          (bind _asscene_component_10 (Utilities|Casting|CastToSceneComponent (Utilities|Array|Get(acopy) (Actor|GetComponentsbyTag "/Script/Engine.ActorComponent" "Pr_N4"))))
          (if _returnvalue_5
            (Game|SpawnActorfromClass _output (Math|Conversions|ToTransform(Vector) (Transformation|GetWorldLocation _asscene_component_10)) "Undefined" "MultiplyWithRoot" 0 0)))
        (:then_4
          (bind _asscene_component_11 (Utilities|Casting|CastToSceneComponent (Utilities|Array|Get(acopy) (Actor|GetComponentsbyTag "/Script/Engine.ActorComponent" "Pr_N5"))))
          (if _returnvalue_5
            (Game|SpawnActorfromClass _output (Math|Conversions|ToTransform(Vector) (Transformation|GetWorldLocation _asscene_component_11)) "Undefined" "MultiplyWithRoot" 0 0)))))))

(fn ConstructionScript)

(fn SpawnMonster
  (bind _returnvalue (Actor|GetComponentsbyTag "/Script/Engine.SceneComponent" "MonsterTriggerPlackart"))
  (bind _output (Utilities|Array|Get(acopy) _returnvalue))
  (bind _returnvalue_2 (Game|SpawnActorfromClass "/Game/InDevelop/Blueprints/BP_MonsterSpawnTrigger.BP_MonsterSpawnTrigger_C" (Math|Transform|MakeTransform (Transformation|GetWorldLocation _output) (Transformation|GetWorldRotation _output)) "AlwaysSpawn" "MultiplyWithRoot" 0 0))
  (Development|PrintString (Utilities|GetDisplayName _returnvalue_2)))