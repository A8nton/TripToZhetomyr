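; Train locomotive actor that sets up its waypoint and handle when play begins.
; BeginPlay finds scene components by the Wp_loc and Hn_loc tags and spawns a Waypoint and a LocoHandle at their world locations.
; The spawned handle is stored in Handle and given a fixed world rotation.
; The FinishTrigger overlap event and construction script are empty.
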(event OnComponentBeginOverlap(FinishTrigger)
  (params (OverlappedComponent :type Primitive%20Component%20Object%20Reference) (OtherActor :type Actor%20Object%20Reference) (OtherComp :type Primitive%20Component%20Object%20Reference) (OtherBodyIndex :type Integer) (bFromSweep :type Boolean) (SweepResult :type Hit%20Result%20Structure%20%28by%20ref%29)))

(event EventBeginPlay
  (Utilities|FlowControl|Sequence
    (:then_0
      (bind _asscene_component (Utilities|Casting|CastToSceneComponent (Utilities|Array|Get(acopy) (Actor|GetComponentsbyTag "/Script/Engine.ActorComponent" "Wp_loc"))))
      (Game|SpawnActorfromClass "/Game/InDevelop/Blueprints/Waypoint.Waypoint_C" (Math|Conversions|ToTransform(Vector) (Transformation|GetWorldLocation _asscene_component)) "Undefined" "MultiplyWithRoot" 0 0))
    (:then_1
      (bind _asscene_component_2 (Utilities|Casting|CastToSceneComponent (Utilities|Array|Get(acopy) (Actor|GetComponentsbyTag "/Script/Engine.ActorComponent" "Hn_loc"))))
      (bind _returnvalue (Game|SpawnActorfromClass "/Game/InDevelop/Blueprints/Meshes/Trains/LocoHandle.LocoHandle_C" (Math|Conversions|ToTransform(Vector) (Transformation|GetWorldLocation _asscene_component_2)) "Undefined" "MultiplyWithRoot" 0 0))
      (bind _output_get (Variables|Default|SetHandle _returnvalue))
      (Transformation|SetActorRotation _output_get "-40.000000,0.000000,0.000000"))))

(fn ConstructionScript)