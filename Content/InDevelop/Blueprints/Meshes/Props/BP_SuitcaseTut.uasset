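; BP_SuitcaseTut is a suitcase prop, apparently for the tutorial, with a waypoint widget that guides the player to it.
; Each tick it shows the player's distance in metres, switching to an interact prompt within 1.5 m.
; Once the suitcase moves fast, the widget switches to world space and is never switched back.
; Fast hits play an impact sound, throttled by a short delay gate.
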(event OnComponentHit(Suitcase)
  (params (HitComponent :type Primitive%20Component%20Object%20Reference) (OtherActor :type Actor%20Object%20Reference) (OtherComp :type Primitive%20Component%20Object%20Reference) (NormalImpulse :type Vector :default "0, 0, 0") (Hit :type Hit%20Result%20Structure%20%28by%20ref%29))
  (bind _audio (Variables|Default|GetAudio))
  (if (> (Math|Vector|VectorLength (Transformation|GetComponentVelocity HitComponent)) 1.5e+02)
    (if (not (Variables|Default|GetIsPlayed))
      (Variables|Default|SetIsPlayed true)
      (Components|Activation|Activate _audio false)
      (Audio|Components|Audio|Play _audio 0.0)
      (Utilities|FlowControl|Delay 0.2)
      (Variables|Default|SetIsPlayed false))))

(event EventBeginPlay
  (bind _asstart_waypoint (Utilities|Casting|CastToStartWaypoint (UserInterface|GetWidget (Variables|Default|GetWidget))))
  (Variables|Components|SetHow%20Long%20Text (Variables|/Game/InDevelop/UI/StartWaypoint.StartWaypoint_C|GetHowLongText _asstart_waypoint)))

(event EventTick
  (params (DeltaSeconds :type Float%20%28single-precision%29))
  (bind _returnvalue (Game|Player|GetPlayerPawn 0))
  (bind _returnvalue_2 (Transformation|GetActorLocation))
  (bind _how_long_text (Variables|Components|GetHow%20Long%20Text))
  (bind _returnvalue_3 (Transformation|GetActorLocation _returnvalue))
  (bind _returnvalue_4 (Math|Vector|Distance(Vector) _returnvalue_2 _returnvalue_3))
  (bind _returnvalue_5 (/ _returnvalue_4 1e+02))
  (Utilities|FlowControl|Sequence
    (:then_0
      (if (<= _returnvalue_5 1.5)
        (Rendering|Components|TextRender|SetText _how_long_text "Press LMB to Interact")
        (else
          (Rendering|Components|TextRender|SetText _how_long_text (Utilities|Text|ToText(String) (Utilities|String|Append (Utilities|String|ToString(Integer) (Math|Float|Truncate _returnvalue_5)) " m"))))))
    (:then_1
      (if (> (Math|Vector|VectorLength (Transformation|GetVelocity self)) 1.5e+02)
        (Class|WidgetComponent|SetWidgetSpace (Variables|Default|GetWidget) "World")))))

(fn ConstructionScript)