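; BP_Suitcase is a suitcase prop that plays an impact sound when it is knocked or dropped with enough force.
; On a component hit of the suitcase, it checks the hit component's velocity against a speed threshold, then activates and plays its audio component.
; A boolean flag with a short delay acts as a cooldown so rapid repeated hits do not retrigger the sound.
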(event OnComponentHit(Suitcase)
  (params (HitComponent :type Primitive%20Component%20Object%20Reference) (OtherActor :type Actor%20Object%20Reference) (OtherComp :type Primitive%20Component%20Object%20Reference) (NormalImpulse :type Vector :default "0, 0, 0") (Hit :type Hit%20Result%20Structure%20%28by%20ref%29))
  (bind _audio (Variables|Default|GetAudio))
  (if (> (Math|Vector|VectorLength (Transformation|GetComponentVelocity HitComponent)) 1.5e+02)
    (if (not (Variables|Default|GetIsPlayed))
      (Variables|Default|SetIsPlayed true)
      (Components|Activation|Activate _audio false)
      (Audio|Components|Audio|Play _audio 0.0)
      (Utilities|FlowControl|Delay 0.2)
      (Variables|Default|SetIsPlayed false))))

(fn ConstructionScript)