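; Boombox prop that plays music on demand and makes impact sounds when knocked around.
; Play and stop events drive the music and switch audio components, with an integer parameter selecting the on or off switch sound.
; Each play attempt on a working boombox has a 1-in-50 chance to trigger a break sound and block further playback.
; Hit sounds require a minimum component velocity and are debounced by a short delay.
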(event OnComponentHit(Boombox)
  (params (HitComponent :type Primitive%20Component%20Object%20Reference) (OtherActor :type Actor%20Object%20Reference) (OtherComp :type Primitive%20Component%20Object%20Reference) (NormalImpulse :type Vector :default "0, 0, 0") (Hit :type Hit%20Result%20Structure%20%28by%20ref%29))
  (bind _au_hit (Variables|Default|GetAu_Hit))
  (if (> (Math|Vector|VectorLength (Transformation|GetComponentVelocity HitComponent)) 1.5e+02)
    (if (not (Variables|Default|GetIsPlayed))
      (Variables|Default|SetIsPlayed true)
      (Components|Activation|Activate _au_hit false)
      (Audio|Components|Audio|Play _au_hit 0.0)
      (Utilities|FlowControl|Delay 0.2)
      (Variables|Default|SetIsPlayed false))))

(event Custom|BoomboxPlay
  (bind _au_music (Variables|Default|GetAu_Music))
  (bind _au_switch (Variables|Default|GetAu_Switch))
  (if (not (Variables|Default|GetisBroken))
    (if (== (Math|Random|RandomIntegerinRange 0 49) 1)
      (Components|Activation|Activate (Variables|Default|GetAu_Break) false)
      (Variables|Default|SetisBroken true)
      (else
        (Components|Activation|Activate _au_switch false)
        (Effects|Components|ParticleSystem|SetIntParameter _au_switch "BoomboxSwitch" 0)
        (Components|Activation|Activate _au_music false)
        (Audio|Components|Audio|Play _au_music 0.0)))))

(event Custom|BoomboxStop
  (bind _au_switch (Variables|Default|GetAu_Switch))
  (Effects|Components|ParticleSystem|SetIntParameter _au_switch "BoomboxSwitch" 1)
  (Audio|Components|Audio|Play _au_switch 0.0)
  (Audio|Components|Audio|Stop (Variables|Default|GetAu_Music)))

(fn ConstructionScript)