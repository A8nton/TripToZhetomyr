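; Train manager that procedurally builds the train one wagon at a time, with scenery and doors, ending in a locomotive.
; BeginPlay spawns the start wagon, moves the player to its tagged spawn point and randomly places props on tagged points.
; SpawnNext disables the last wagon's trigger and attaches a random Intercity, Coupe or Plackart wagon using front/back spawn points.
; Per-type counters limit repeats; once the wagon quota is reached, it spawns the locomotive and fog.
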(event Custom|SpawnNext
  (CallFunction|SpNextWagon))

(event EventBeginPlay
  (Utilities|FlowControl|Sequence
    (:then_0
      (CallFunction|SpInitialWagon))
    (:then_1
      (Default|GetManager (Variables|Default|GetLastSpawnedWagon) self))))

(fn ConstructionScript)

(fn SpInitialWagon
  (bind _returnvalue (Math|Random|RandomIntegerinRange 0 2))
  (bind _returnvalue_2 (Math|Random|RandomIntegerinRange 0 3))
  (bind _spawnablepropsn (Variables|Default|GetSpawnablePropsN))
  (bind _spawncoordinates (LocalVariables|GetSpawnCoordinates))
  (bind _output (Utilities|Array|Get(acopy) _spawnablepropsn _returnvalue_2))
  (bind _returnvalue_3 (== _returnvalue 1))
  (Utilities|FlowControl|Sequence
    (:then_0
      (Development|PrintText "launched")
      (bind _returnvalue_4 (Game|SpawnActorfromClass "/Game/InDevelop/Blueprints/Meshes/Trains/BP_TrainStart.BP_TrainStart_C" _spawncoordinates "Undefined" "MultiplyWithRoot" 0 0))
      (Utilities|FlowControl|Sequence
        (:then_0
          (bind _output_get (Variables|Default|SetLastSpawnedWagon _returnvalue_4))
          (Utilities|Array|Add (Variables|Default|GetSpawnedTrainWagons) _output_get)
          (Default|GetManager _output_get self)
          (Actor|GetAllActorsOfClass "/Game/InDevelop/Blueprints/Meshes/Trains/BP_TrainBase.BP_TrainBase_C")
          (bind _asscene_component (Utilities|Casting|CastToSceneComponent (Utilities|Array|Get(acopy) (Actor|GetComponentsbyTag _returnvalue_4 "/Script/Engine.ActorComponent" "PlayerSpawn"))))
          (Transformation|SetActorLocation (Game|GetPlayerCharacter 0) (Transformation|GetWorldLocation _asscene_component) false false)
          (Game|SpawnActorfromClass "/Game/InDevelop/Blueprints/Meshes/Nature/Nature.Nature_C" (Math|Conversions|ToTransform(Vector) (- (Transformation|GetWorldLocation (Variables|/Game/InDevelop/Blueprints/Meshes/Trains/BP_TrainBase.BP_TrainBase_C|GetFrontSpawnPoint (Variables|Default|GetLastSpawnedWagon))) (Variables|/Script/Engine.SceneComponent|GetRelativeLocation (Variables|/Game/InDevelop/Blueprints/Meshes/Trains/BP_TrainBase.BP_TrainBase_C|GetBackSpawnPoint (Variables|Default|GetLastSpawnedWagon))))) "Undefined" "MultiplyWithRoot" 0 0)
          (Game|SpawnActorfromClass "/Game/InDevelop/Blueprints/Meshes/Trains/BP_TrainDoorEntr.BP_TrainDoorEntr_C" (LocalVariables|GetSpawnCoordinates) "Undefined" "MultiplyWithRoot" 0 0)
          (Game|SpawnActorfromClass "/Game/InDevelop/Blueprints/Meshes/Trains/BP_TrainDoorEntr.BP_TrainDoorEntr_C" (Math|Conversions|ToTransform(Vector) (- (Transformation|GetWorldLocation (Variables|/Game/InDevelop/Blueprints/Meshes/Trains/BP_TrainBase.BP_TrainBase_C|GetFrontSpawnPoint (Variables|Default|GetLastSpawnedWagon))) (Variables|/Script/Engine.SceneComponent|GetRelativeLocation (Variables|/Game/InDevelop/Blueprints/Meshes/Trains/BP_TrainBase.BP_TrainBase_C|GetBackSpawnPoint (Variables|Default|GetLastSpawnedWagon))))) "Undefined" "MultiplyWithRoot" 0 0)
          (Game|SpawnActorfromClass "/Game/InDevelop/Blueprints/Meshes/Nature/Nature.Nature_C" (Math|Conversions|ToTransform(Vector) (- (Variables|/Script/Engine.SceneComponent|GetRelativeLocation (Variables|/Game/InDevelop/Blueprints/Meshes/Trains/BP_TrainBase.BP_TrainBase_C|GetBackSpawnPoint (Variables|Default|GetLastSpawnedWagon))) (Transformation|GetWorldLocation (Variables|/Game/InDevelop/Blueprints/Meshes/Trains/BP_TrainBase.BP_TrainBase_C|GetFrontSpawnPoint (Variables|Default|GetLastSpawnedWagon))))) "Undefined" "MultiplyWithRoot" 0 0))))
    (:then_1
      (Game|SpawnActorfromClass "/Game/InDevelop/Blueprints/Meshes/Nature/Nature.Nature_C" _spawncoordinates "Undefined" "MultiplyWithRoot" 0 0))
    (:then_2
      (Utilities|FlowControl|Sequence
        (:then_0
          (|RandomUselessspawn _returnvalue_4 :!label _label))
        (:then_1
          (goto _label execute3))
        (:then_2
          (goto _label execute4))
        (:then_3
          (goto _label execute5))
        (:then_4
          (goto _label execute6))
        (:then_5
          (goto _label execute2))
        (:then_6
          (Utilities|FlowControl|Sequence
            (:then_0
              (bind _asscene_component_2 (Utilities|Casting|CastToSceneComponent (Utilities|Array|Get(acopy) (Actor|GetComponentsbyTag _returnvalue_4 "/Script/Engine.ActorComponent" "Pr_N1"))))
              (if _returnvalue_3
                (Game|SpawnActorfromClass _output (Math|Conversions|ToTransform(Vector) (Transformation|GetWorldLocation _asscene_component_2)) "Undefined" "MultiplyWithRoot" 0 0)))
            (:then_1
              (bind _asscene_component_3 (Utilities|Casting|CastToSceneComponent (Utilities|Array|Get(acopy) (Actor|GetComponentsbyTag _returnvalue_4 "/Script/Engine.ActorComponent" "Pr_N2"))))
              (if _returnvalue_3
                (Game|SpawnActorfromClass _output (Math|Conversions|ToTransform(Vector) (Transformation|GetWorldLocation _asscene_component_3)) "Undefined" "MultiplyWithRoot" 0 0)))))))))

(fn SpNextWagon
  (CallFunction|DisableTrigger)
  (Utilities|FlowControl|Sequence
    (:then_0
      (if (< (Variables|Default|GetTotalCountOfWagons) (Variables|Default|GetNeededWagonsBeforeLoco))
        (switch int (CallFunction|GenerateRandomNum)
          (:0
            (bind _returnvalue (Game|SpawnActorfromClass "/Game/InDevelop/Blueprints/Meshes/Trains/BP_TrainIntercity.BP_TrainIntercity_C" (Math|Conversions|ToTransform(Vector) (- (Transformation|GetWorldLocation (Variables|/Game/InDevelop/Blueprints/Meshes/Trains/BP_TrainBase.BP_TrainBase_C|GetFrontSpawnPoint (Variables|Default|GetLastSpawnedWagon))) (Variables|/Script/Engine.SceneComponent|GetRelativeLocation (Variables|/Game/InDevelop/Blueprints/Meshes/Trains/BP_TrainBase.BP_TrainBase_C|GetBackSpawnPoint (Variables|Default|GetLastSpawnedWagon))))) "Undefined" "MultiplyWithRoot" 0 0))
            (bind _output_get (Variables|Default|SetLastSpawnedWagon _returnvalue))
            (Default|GetManager _output_get self)
            (Variables|Default|SetIntercityAntiAgain (+ (Variables|Default|GetIntercityAntiAgain) 1))
            (Utilities|Array|Add (Variables|Default|GetSpawnedTrainWagons) _output_get)
            (Development|PrintString "Spawned Next" :!label _label)
            (Variables|Default|SetTotalCountOfWagons (+ (Variables|Default|GetTotalCountOfWagons) 1))
            (Development|PrintString (Utilities|String|ToString(Integer) (Variables|Default|GetIntercityAntiAgain)))
            (Development|PrintString (Utilities|String|ToString(Integer) (Variables|Default|GetCoupeAntiAgain)))
            (Development|PrintString (Utilities|String|ToString(Integer) (Variables|Default|GetPlackartAntiAgain))))
          (:1
            (bind _returnvalue_2 (Game|SpawnActorfromClass "/Game/InDevelop/Blueprints/Meshes/Trains/BP_TrainCoupe.BP_TrainCoupe_C" (Math|Conversions|ToTransform(Vector) (- (Transformation|GetWorldLocation (Variables|/Game/InDevelop/Blueprints/Meshes/Trains/BP_TrainBase.BP_TrainBase_C|GetFrontSpawnPoint (Variables|Default|GetLastSpawnedWagon))) (Variables|/Script/Engine.SceneComponent|GetRelativeLocation (Variables|/Game/InDevelop/Blueprints/Meshes/Trains/BP_TrainBase.BP_TrainBase_C|GetBackSpawnPoint (Variables|Default|GetLastSpawnedWagon))))) "Undefined" "MultiplyWithRoot" 0 0))
            (Utilities|FlowControl|Sequence
              (:then_0
                (Game|SpawnActorfromClass "/Game/InDevelop/Blueprints/Meshes/Trains/BP_TrainDoorCoupe.BP_TrainDoorCoupe_C" (Math|Conversions|ToTransform(Vector) (- (Transformation|GetWorldLocation (Variables|/Game/InDevelop/Blueprints/Meshes/Trains/BP_TrainBase.BP_TrainBase_C|GetFrontSpawnPoint (Variables|Default|GetLastSpawnedWagon))) (Variables|/Script/Engine.SceneComponent|GetRelativeLocation (Variables|/Game/InDevelop/Blueprints/Meshes/Trains/BP_TrainBase.BP_TrainBase_C|GetBackSpawnPoint (Variables|Default|GetLastSpawnedWagon))))) "Undefined" "MultiplyWithRoot" 0 0))
              (:then_1
                (bind _output_get_2 (Variables|Default|SetLastSpawnedWagon _returnvalue_2))
                (Default|GetManager _output_get_2 self)
                (Variables|Default|SetCoupeAntiAgain (+ (Variables|Default|GetCoupeAntiAgain) 1))
                (Utilities|Array|Add (Variables|Default|GetSpawnedTrainWagons) _output_get_2)
                (goto _label))))
          (:2
            (bind _returnvalue_3 (Game|SpawnActorfromClass "/Game/InDevelop/Blueprints/Meshes/Trains/BP_TrainPlackart.BP_TrainPlackart_C" (Math|Conversions|ToTransform(Vector) (- (Transformation|GetWorldLocation (Variables|/Game/InDevelop/Blueprints/Meshes/Trains/BP_TrainBase.BP_TrainBase_C|GetFrontSpawnPoint (Variables|Default|GetLastSpawnedWagon))) (Variables|/Script/Engine.SceneComponent|GetRelativeLocation (Variables|/Game/InDevelop/Blueprints/Meshes/Trains/BP_TrainBase.BP_TrainBase_C|GetBackSpawnPoint (Variables|Default|GetLastSpawnedWagon))))) "Undefined" "MultiplyWithRoot" 0 0))
            (bind _output_get_3 (Variables|Default|SetLastSpawnedWagon _returnvalue_3))
            (Default|GetManager _output_get_3 self)
            (Variables|Default|SetPlackartAntiAgain (+ (Variables|Default|GetPlackartAntiAgain) 1))
            (Utilities|Array|Add (Variables|Default|GetSpawnedTrainWagons) _output_get_3)
            (goto _label)))
        (else
          (bind _returnvalue_4 (Game|SpawnActorfromClass "/Game/InDevelop/Blueprints/Meshes/Trains/BP_TrainLoco.BP_TrainLoco_C" (Math|Conversions|ToTransform(Vector) (- (Transformation|GetWorldLocation (Variables|/Game/InDevelop/Blueprints/Meshes/Trains/BP_TrainBase.BP_TrainBase_C|GetFrontSpawnPoint (Variables|Default|GetLastSpawnedWagon))) (Variables|/Script/Engine.SceneComponent|GetRelativeLocation (Variables|/Game/InDevelop/Blueprints/Meshes/Trains/BP_TrainBase.BP_TrainBase_C|GetBackSpawnPoint (Variables|Default|GetLastSpawnedWagon))))) "Undefined" "MultiplyWithRoot" 0 0))
          (bind _output_get_4 (Variables|Default|SetLastSpawnedWagon _returnvalue_4))
          (Default|GetManager _output_get_4 self)
          (CallFunction|DisableTrigger))))
    (:then_1
      (if (< (Variables|Default|GetTotalCountOfWagons) (Variables|Default|GetNeededWagonsBeforeLoco))
        (Game|SpawnActorfromClass "/Game/InDevelop/Blueprints/Meshes/Nature/Nature.Nature_C" (Math|Conversions|ToTransform(Vector) (- (Transformation|GetWorldLocation (Variables|/Game/InDevelop/Blueprints/Meshes/Trains/BP_TrainBase.BP_TrainBase_C|GetFrontSpawnPoint (Variables|Default|GetLastSpawnedWagon))) (Variables|/Script/Engine.SceneComponent|GetRelativeLocation (Variables|/Game/InDevelop/Blueprints/Meshes/Trains/BP_TrainBase.BP_TrainBase_C|GetBackSpawnPoint (Variables|Default|GetLastSpawnedWagon))))) "Undefined" "MultiplyWithRoot" 0 0)
        (Game|SpawnActorfromClass "/Game/InDevelop/Blueprints/Meshes/Trains/BP_TrainDoorEntr.BP_TrainDoorEntr_C" (Math|Conversions|ToTransform(Vector) (- (Transformation|GetWorldLocation (Variables|/Game/InDevelop/Blueprints/Meshes/Trains/BP_TrainBase.BP_TrainBase_C|GetFrontSpawnPoint (Variables|Default|GetLastSpawnedWagon))) (Variables|/Script/Engine.SceneComponent|GetRelativeLocation (Variables|/Game/InDevelop/Blueprints/Meshes/Trains/BP_TrainBase.BP_TrainBase_C|GetBackSpawnPoint (Variables|Default|GetLastSpawnedWagon))))) "Undefined" "MultiplyWithRoot" 0 0)
        (else
          (Game|SpawnActorfromClass "/Game/InDevelop/Blueprints/Meshes/Nature/Nature.Nature_C" (Math|Conversions|ToTransform(Vector) (- (Transformation|GetWorldLocation (Variables|/Game/InDevelop/Blueprints/Meshes/Trains/BP_TrainBase.BP_TrainBase_C|GetFrontSpawnPoint (Variables|Default|GetLastSpawnedWagon))) (Variables|/Script/Engine.SceneComponent|GetRelativeLocation (Variables|/Game/InDevelop/Blueprints/Meshes/Trains/BP_TrainBase.BP_TrainBase_C|GetBackSpawnPoint (Variables|Default|GetLastSpawnedWagon))))) "Undefined" "MultiplyWithRoot" 0 0)
          (Game|SpawnActorfromClass "/Game/InDevelop/Blueprints/Meshes/Nature/NatureFog.NatureFog_C" (Math|Conversions|ToTransform(Vector) (- (Transformation|GetWorldLocation (Variables|/Game/InDevelop/Blueprints/Meshes/Trains/BP_TrainBase.BP_TrainBase_C|GetFrontSpawnPoint (Variables|Default|GetLastSpawnedWagon))) (Variables|/Script/Engine.SceneComponent|GetRelativeLocation (Variables|/Game/InDevelop/Blueprints/Meshes/Trains/BP_TrainBase.BP_TrainBase_C|GetBackSpawnPoint (Variables|Default|GetLastSpawnedWagon))))) "Undefined" "MultiplyWithRoot" 0 0))))))

(fn DisableTrigger
  (Collision|SetCollisionEnabled (Variables|/Game/InDevelop/Blueprints/Meshes/Trains/BP_TrainBase.BP_TrainBase_C|GetSpawnTrigger (Variables|Default|GetLastSpawnedWagon)) "NoCollision"))

(fn GenerateRandomNum
  (bind _output_get (Variables|Default|SetRandomWagonNumber (Math|Random|RandomIntegerinRange 0 2)))
  (switch int _output_get
    (:0
      (if (== (Variables|Default|GetIntercityAntiAgain) 2)
        (Variables|Default|SetRandomWagonNumber 1)
        (Variables|Default|SetIntercityAntiAgain 0)
        (else
          (Variables|Default|SetCoupeAntiAgain 0)
          (Variables|Default|SetPlackartAntiAgain 0))))
    (:1
      (if (== (Variables|Default|GetCoupeAntiAgain) 2)
        (Variables|Default|SetRandomWagonNumber 2)
        (Variables|Default|SetPlackartAntiAgain 0)
        (else
          (Variables|Default|SetIntercityAntiAgain 0)
          (Variables|Default|SetPlackartAntiAgain 0))))
    (:2
      (if (== (Variables|Default|GetPlackartAntiAgain) 2)
        (Variables|Default|SetRandomWagonNumber 0)
        (Variables|Default|SetRandomWagonNumber 0)
        (else
          (Variables|Default|SetIntercityAntiAgain 0)
          (Variables|Default|SetCoupeAntiAgain 0)))))
  (return (Variables|Default|GetRandomWagonNumber)))