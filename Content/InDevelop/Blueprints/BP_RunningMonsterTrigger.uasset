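; BP_RunningMonsterTrigger is an overlap trigger that spawns running monsters in train coupes when the player enters it.
; It loops over TrainCoupe-tagged actors, using tagged scene components as spawn points.
; The first pass spawns a monster, then after a Delay spawns another and removes the coupe's MonsterTrigger component.
; Any pass with the spawn flag already set, including later loop iterations, destroys the trigger and first monster.
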(event Collision|EventActorBeginOverlap
  (params (OtherActor :type Actor%20Object%20Reference))
  (bind _outactors (Actor|GetAllActorswithTag "TrainCoupe"))
  (bind _output_get (Variables|Default|SetArray _outactors))
  (for _array_element _output_get
    (bind _output_get_2 (Variables|Default|SetActorElement _array_element))
    (if (== OtherActor (Game|GetPlayerCharacter 0))
      (if (Variables|Default|GetbIsMonsterSpawn)
        (Actor|DestroyActor)
        (Actor|DestroyActor (stale _returnvalue))
        (else
          (bind _returnvalue (Game|SpawnActorfromClass "/Game/InDevelop/Blueprints/BP_RunningMonster.BP_RunningMonster_C" (Math|Transform|MakeTransform (Transformation|GetWorldLocation (Utilities|Array|Get(acopy) (Actor|GetComponentsbyTag _output_get_2 "/Script/Engine.SceneComponent" "Monster"))) (Transformation|GetWorldRotation (Utilities|Array|Get(acopy) (Actor|GetComponentsbyTag _output_get_2 "/Script/Engine.SceneComponent" "Monster")))) "AlwaysSpawn" "MultiplyWithRoot" 0 0))
          (Variables|Default|SetMonstr _returnvalue)
          (Variables|Default|SetbIsMonsterSpawn true)
          (Utilities|FlowControl|Delay 5.0)
          (Game|SpawnActorfromClass "/Game/InDevelop/Blueprints/BP_RunningMonster.BP_RunningMonster_C" (Math|Transform|MakeTransform (Transformation|GetWorldLocation (Utilities|Array|Get(acopy) (Actor|GetComponentsbyTag _output_get_2 "/Script/Engine.SceneComponent" "MonsterCoupe"))) (Transformation|GetWorldRotation (Utilities|Array|Get(acopy) (Actor|GetComponentsbyTag _output_get_2 "/Script/Engine.SceneComponent" "MonsterCoupe")))) "Undefined" "MultiplyWithRoot" 0 0)
          (Components|DestroyComponent (Utilities|Array|Get(acopy) (Actor|GetComponentsbyTag _output_get_2 "/Script/Engine.SceneComponent" "MonsterTrigger"))))))))

(fn ConstructionScript)