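; BP_Plank is a final-puzzle plank actor that plays a break cinematic and opens the train exit.
; It registers itself with the player character on BeginPlay and receives its TrainFin reference through GetTrainFin.
; PlayBreak starts the sequence and blends the camera to the plank, then after a fixed delay returns the view and disables ExitBlock collision on TrainFin.
; A sequencer event triggers the audio.
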(event Custom|PlayBreak
  (bind _returnvalue (Game|GetPlayerController 0))
  (Class|ActorSequenceComponent|PlaySequence (Variables|Default|GetBreakSequence))
  (Game|Player|SetViewTargetwithBlend _returnvalue self 0.5 "VTBlend_Linear" 0.0 false)
  (Utilities|FlowControl|Delay 11.0)
  (bind _asbp_fps_character_dev (Utilities|Casting|CastToBP_FPS_Character_Dev (Game|GetPlayerCharacter 0)))
  (Game|Player|SetViewTargetwithBlend _returnvalue _asbp_fps_character_dev 0.5 "VTBlend_Linear" 0.0 false)
  (Collision|SetCollisionEnabled (Variables|/Game/InDevelop/Blueprints/Puzzles/FinalPuzzle/BP_TrainFin.BP_TrainFin_C|GetExitBlock (Variables|Default|GetTrainFin)) "NoCollision"))

(event Custom|GetTrainFin
  (params (TrainFin :type BP%20Train%20Fin%20Object%20Reference))
  (Variables|Default|SetTrainFin TrainFin))

(event EventBeginPlay
  (bind _asbp_fps_character_dev (Utilities|Casting|CastToBP_FPS_Character_Dev (Game|GetPlayerCharacter 0)))
  (Default|GetPlanks _asbp_fps_character_dev self))

(event Custom|SequenceEvent
  (Audio|Components|Audio|Play (Variables|Default|GetAudio) 0.0))

(fn ConstructionScript)