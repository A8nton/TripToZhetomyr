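; One-shot trigger that populates train compartments with doors, notes and a monster threat when the player overlaps it.
; It finds TrainCoupe actors and spawns a locked door, steel door and four notes at their tagged components.
; It removes any monster flagged Spawned and destroys itself.
; A parallel 60-second delay is meant to swap the steel door for BP_Monster, but the trigger destroys itself before that delay ends.
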(event Collision|EventActorBeginOverlap
  (params (OtherActor :type Actor%20Object%20Reference))
  (Utilities|FlowControl|Delay 0.2)
  (bind _outactors (Actor|GetAllActorswithTag "TrainCoupe"))
  (bind _output_get (Variables|Default|SetArray _outactors))
  (for _array_element _output_get
    (if (== OtherActor (Game|GetPlayerCharacter 0))
      (Utilities|FlowControl|Sequence
        (:then_0
          (bind _output_get_2 (Variables|Default|SetIs%20spawned false))
          (if (not _output_get_2)
            (Game|SpawnActorfromClass "/Game/InDevelop/Blueprints/Puzzles/LockDoor/BP_door.BP_door_C" (Math|Transform|MakeTransform (+ (.Location (Math|Transform|BreakTransform (Math|Transform|MakeTransform (Transformation|GetWorldLocation (Utilities|Array|Get(acopy) (Actor|GetComponentsbyTag _array_element "/Script/Engine.SceneComponent" "DoorWithLock"))) (Transformation|GetWorldRotation (Utilities|Array|Get(acopy) (Actor|GetComponentsbyTag _array_element "/Script/Engine.SceneComponent" "DoorWithLock")))))) "0.000000,0.000000,100.000000") (.Rotation (Math|Transform|BreakTransform (Math|Transform|MakeTransform (Transformation|GetWorldLocation (Utilities|Array|Get(acopy) (Actor|GetComponentsbyTag _array_element "/Script/Engine.SceneComponent" "DoorWithLock"))) (Transformation|GetWorldRotation (Utilities|Array|Get(acopy) (Actor|GetComponentsbyTag _array_element "/Script/Engine.SceneComponent" "DoorWithLock")))))) (.Scale (Math|Transform|BreakTransform (Math|Transform|MakeTransform (Transformation|GetWorldLocation (Utilities|Array|Get(acopy) (Actor|GetComponentsbyTag _array_element "/Script/Engine.SceneComponent" "DoorWithLock"))) (Transformation|GetWorldRotation (Utilities|Array|Get(acopy) (Actor|GetComponentsbyTag _array_element "/Script/Engine.SceneComponent" "DoorWithLock"))))))) "AlwaysSpawn" "MultiplyWithRoot" 0 0)
            (Variables|Default|SetIs%20spawned true)
            (Utilities|FlowControl|Delay 0.5)
            (Game|SpawnActorfromClass "/Game/InDevelop/Blueprints/Puzzles/LockDoor/BP_SteelDoor.BP_SteelDoor_C" (Math|Transform|MakeTransform (+ (.Location (Math|Transform|BreakTransform (Math|Transform|MakeTransform (Transformation|GetWorldLocation (Utilities|Array|Get(acopy) (Actor|GetComponentsbyTag _array_element "/Script/Engine.SceneComponent" "SteelDoor"))) (Transformation|GetWorldRotation (Utilities|Array|Get(acopy) (Actor|GetComponentsbyTag _array_element "/Script/Engine.SceneComponent" "SteelDoor")))))) "0.000000,0.000000,100.000000") (.Rotation (Math|Transform|BreakTransform (Math|Transform|MakeTransform (Transformation|GetWorldLocation (Utilities|Array|Get(acopy) (Actor|GetComponentsbyTag _array_element "/Script/Engine.SceneComponent" "SteelDoor"))) (Transformation|GetWorldRotation (Utilities|Array|Get(acopy) (Actor|GetComponentsbyTag _array_element "/Script/Engine.SceneComponent" "SteelDoor")))))) (.Scale (Math|Transform|BreakTransform (Math|Transform|MakeTransform (Transformation|GetWorldLocation (Utilities|Array|Get(acopy) (Actor|GetComponentsbyTag _array_element "/Script/Engine.SceneComponent" "SteelDoor"))) (Transformation|GetWorldRotation (Utilities|Array|Get(acopy) (Actor|GetComponentsbyTag _array_element "/Script/Engine.SceneComponent" "SteelDoor"))))))) "Undefined" "MultiplyWithRoot" 0 0)
            (bind _returnvalue (Actor|GetActorOfClass "/Game/InDevelop/Blueprints/BP_Monster.BP_Monster_C"))
            (for _array_element_2 (Variables|Default|GetArray)
              (Variables|Default|SetArrayElment _array_element_2)
              (Actor|DestroyActor)
              (Utilities|FlowControl|Sequence
                (:then_0
                  (bind _returnvalue_2 (CallFunction|SetTransformOne))
                  (Game|SpawnActorfromClass "/Game/InDevelop/Blueprints/Puzzles/LockDoor/BP_Note1.BP_Note1_C" _returnvalue_2 "Undefined" "MultiplyWithRoot" 0 0))
                (:then_1
                  (bind _returnvalue_3 (CallFunction|SetTransformTwo))
                  (Game|SpawnActorfromClass "/Game/InDevelop/Blueprints/Puzzles/LockDoor/BP_Note2.BP_Note2_C" _returnvalue_3 "Undefined" "MultiplyWithRoot" 0 0))
                (:then_2
                  (bind _returnvalue_4 (CallFunction|SetTransformThree))
                  (Game|SpawnActorfromClass "/Game/InDevelop/Blueprints/Puzzles/LockDoor/BP_Note3.BP_Note3_C" _returnvalue_4 "Undefined" "MultiplyWithRoot" 0 0))
                (:then_3
                  (bind _returnvalue_5 (CallFunction|SetTransformFour))
                  (Game|SpawnActorfromClass "/Game/InDevelop/Blueprints/Puzzles/LockDoor/BP_Note4.BP_Note4_C" _returnvalue_5 "Undefined" "MultiplyWithRoot" 0 0)))
              (if (Variables|/Game/InDevelop/Blueprints/BP_Monster.BP_Monster_C|GetSpawned _returnvalue)
                (Actor|DestroyActor _returnvalue)))))
        (:then_1
          (Utilities|FlowControl|Delay 6e+01)
          (bind _returnvalue_6 (Actor|GetActorOfClass "/Game/InDevelop/Blueprints/Puzzles/LockDoor/BP_SteelDoor.BP_SteelDoor_C"))
          (Actor|DestroyActor _returnvalue_6)
          (Game|SpawnActorfromClass "/Game/InDevelop/Blueprints/BP_Monster.BP_Monster_C" (Math|Transform|MakeTransform (Transformation|GetWorldLocation (Utilities|Array|Get(acopy) (Actor|GetComponentsbyTag _array_element "/Script/Engine.SceneComponent" "SteelDoor"))) (Transformation|GetWorldRotation (Utilities|Array|Get(acopy) (Actor|GetComponentsbyTag _array_element "/Script/Engine.SceneComponent" "SteelDoor")))) "AlwaysSpawn" "MultiplyWithRoot" 0 0))))))

(fn ConstructionScript)

(fn SetTransformOne
  (bind _arrayelment (Variables|Default|GetArrayElment))
  (bind _returnvalue (Actor|GetComponentsbyTag _arrayelment "/Script/Engine.SceneComponent" "Note1"))
  (bind _output (Utilities|Array|Get(acopy) _returnvalue))
  (bind _returnvalue_2 (Transformation|GetWorldRotation _output))
  (bind _returnvalue_3 (Transformation|GetWorldLocation _output))
  (bind _returnvalue_4 (Math|Transform|MakeTransform _returnvalue_3 _returnvalue_2))
  (bind (_location _rotation _scale) (Math|Transform|BreakTransform _returnvalue_4))
  (return (Math|Transform|MakeTransform _location _rotation _scale)))

(fn SetTransformTwo
  (bind _arrayelment (Variables|Default|GetArrayElment))
  (bind _returnvalue (Actor|GetComponentsbyTag _arrayelment "/Script/Engine.SceneComponent" "Note2"))
  (bind _output (Utilities|Array|Get(acopy) _returnvalue))
  (bind _returnvalue_2 (Transformation|GetWorldLocation _output))
  (bind _returnvalue_3 (Transformation|GetWorldRotation _output))
  (bind _returnvalue_4 (Math|Transform|MakeTransform _returnvalue_2 _returnvalue_3))
  (bind (_location _rotation _scale) (Math|Transform|BreakTransform _returnvalue_4))
  (return (Math|Transform|MakeTransform _location _rotation _scale)))

(fn SetTransformThree
  (bind _arrayelment (Variables|Default|GetArrayElment))
  (bind _returnvalue (Actor|GetComponentsbyTag _arrayelment "/Script/Engine.SceneComponent" "Note3"))
  (bind _output (Utilities|Array|Get(acopy) _returnvalue))
  (bind _returnvalue_2 (Transformation|GetWorldRotation _output))
  (bind _returnvalue_3 (Transformation|GetWorldLocation _output))
  (bind _returnvalue_4 (Math|Transform|MakeTransform _returnvalue_3 _returnvalue_2))
  (bind (_location _rotation _scale) (Math|Transform|BreakTransform _returnvalue_4))
  (return (Math|Transform|MakeTransform _location _rotation _scale)))

(fn SetTransformFour
  (bind _arrayelment (Variables|Default|GetArrayElment))
  (bind _returnvalue (Actor|GetComponentsbyTag _arrayelment "/Script/Engine.SceneComponent" "Note4"))
  (bind _output (Utilities|Array|Get(acopy) _returnvalue))
  (bind _returnvalue_2 (Transformation|GetWorldRotation _output))
  (bind _returnvalue_3 (Transformation|GetWorldLocation _output))
  (bind _returnvalue_4 (Math|Transform|MakeTransform _returnvalue_3 _returnvalue_2))
  (bind (_location _rotation _scale) (Math|Transform|BreakTransform _returnvalue_4))
  (return (Math|Transform|MakeTransform _location _rotation _scale)))